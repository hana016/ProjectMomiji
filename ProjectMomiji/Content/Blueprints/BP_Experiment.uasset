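; BP_Experiment is a bare experiment Blueprint, apparently meant as a base class, that tracks whether an experiment is active and how it finishes.
; Activate and deactivate events set the active flag, then call empty OnActivateExperiment and OnDeactivateExperiment hooks.
; The success and failure finish events each call their matching Finished dispatcher, then deactivate the experiment.
; Two debug prints for the outcomes are left unconnected and never run.
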(event Custom|ActivateExperiment
  (Variables|Default|SetisExperimentActive true)
  (CallFunction|OnActivateExperiment))

(event Custom|DeactivateExperiment
  (Variables|Default|SetisExperimentActive false)
  (CallFunction|OnDeactivateExperiment))

(event Custom|OnActivateExperiment)

(event Custom|OnDeactivateExperiment)

(event Custom|FinishSuccessfully
  (Default|CallFinishedSuccessfully)
  (CallFunction|DeactivateExperiment))

(event Custom|FinishUnsuccessfully
  (Default|CallFinishedUnsuccessfully)
  (CallFunction|DeactivateExperiment))

(fn ConstructionScript)