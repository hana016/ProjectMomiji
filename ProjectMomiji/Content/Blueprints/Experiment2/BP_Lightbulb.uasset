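; BP_Lightbulb is an interactive bulb in Experiment2 that acts as a binary digit, starting with its point light hidden.
; Touch and mouse press both toggle the light, play a plop sound and call HasBeenTouched.
; Toggling updates the DisplayValue widget to 1 or 0 alongside the light.
; SetLight reuses the same on and off branches to force a state without the sound or touch call.
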(event Custom|ToggleLight
  (if (Variables|Default|GetisLightOn)
    (Variables|Default|SetisLightOn false)
    (Development|SetHiddeninGame (Variables|Default|GetPointLight) true false)
    (Default|ChangeValue (Variables|Default|GetBinaryValueWidget) 0.0)
    (else
      (Variables|Default|SetisLightOn true)
      (Development|SetHiddeninGame (Variables|Default|GetPointLight) false false)
      (Default|ChangeValue (Variables|Default|GetBinaryValueWidget) 1.0))))

(event Custom|SetLight
  (params (isOn :type Boolean))
  (if isOn
    (Variables|Default|SetisLightOn true)
    (Development|SetHiddeninGame (Variables|Default|GetPointLight) false false)
    (Default|ChangeValue (Variables|Default|GetBinaryValueWidget) 1.0)
    (else
      (Variables|Default|SetisLightOn false)
      (Development|SetHiddeninGame (Variables|Default|GetPointLight) true false)
      (Default|ChangeValue (Variables|Default|GetBinaryValueWidget) 0.0))))

(event EventBeginPlay
  (Development|SetHiddeninGame (Variables|Default|GetPointLight) true false)
  (bind _asdisplay_value (Utilities|Casting|CastToDisplayValue (UserInterface|GetWidget (Variables|Default|GetValue))))
  (Variables|Default|SetBinaryValueWidget _asdisplay_value))

(event EventMouseTouch
  (CallFunction|ToggleLight)
  (Audio|PlaySound2D "/Game/Sounds/Plopp.Plopp" 1.0 1.0 0.0 0 0)
  (Default|CallHasBeenTouched))

(event EventMouseTouchRelease)

(event EventTouchInteract
  (params (Location :type Vector :default "0, 0, 0"))
  (CallFunction|ToggleLight)
  (Audio|PlaySound2D "/Game/Sounds/Plopp.Plopp" 1.0 1.0 0.0 0 0)
  (Default|CallHasBeenTouched))

(fn ConstructionScript)