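; Binary-number experiment in which the player toggles lightbulbs, each one a bit, to form random target numbers.
; Every touch updates binary and decimal displays, spends a touch from a limited budget and checks the powers-of-two sum against the target.
; Difficulty sets number range and touch budget.
; Enough correct answers finish the experiment successfully; exhausting touches fails it, with progress shown through an instruction widget.
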(event Custom|CheckIfNumberIsCorrect
  (bind _numberofmaxtouches (Variables|Default|GetNumberOfMaxTouches))
  (bind _binarnumber (CallFunction|GetBinaryNumberfromTorches))
  (Default|ChangeValue (Variables|Default|GetBinaryDisplay) (Math|Conversions|ToFloat(Integer) _binarnumber))
  (bind _decimalnumber (CallFunction|GetDecimalNumberfromTorches))
  (Default|ChangeValue (Variables|Default|GetDecimalDisplay) (Math|Conversions|ToFloat(Integer) _decimalnumber))
  (if (Variables|Default|GetisExperimentActive)
    (if (<= _numberofmaxtouches 0)
      (CallFunction|FinishUnsuccessfully)
      (else
        (Math|Integer|DecrementInt _numberofmaxtouches
          (:%20%20
            (Default|SetBinaryInformation (Variables|Default|GetUIBinaryInstruction) (Variables|Default|GetRandomNumber) (Variables|Default|GetNumberOfMaxTouches))
            (bind _iscorrect (CallFunction|CheckforCorrectBinaryNumber))
            (if _iscorrect
              (CallFunction|SetMaxTouches)
              (Math|Integer|IncrementInt (Variables|Default|GetNumberOfCorrectAnswers)
                (:%20%20
                  (CallFunction|GetRandomNumber)))
              (elif (<= (Variables|Default|GetNumberOfMaxTouches) 0)
                (CallFunction|FinishUnsuccessfully)))))))))

(event Custom|GetRandomNumber
  (if (< (Variables|Default|GetNumberOfCorrectAnswers) (Variables|Default|GetNumberOfNeededCorrectAnswers))
    (if (== (Variables|Default|GetNumberOfCorrectAnswers) 0)
      _
      (else
        (Utilities|FlowControl|Delay 1.0)))
    (CallFunction|SwitchOffAllLightbulbs)
    (CallFunction|GetNewRandomNumber)
    (Default|SetBinaryInformation (Variables|Default|GetUIBinaryInstruction) (Variables|Default|GetRandomNumber) (Variables|Default|GetNumberOfMaxTouches))
    (else
      (Utilities|FlowControl|Delay 1.0)
      (CallFunction|FinishSuccessfully))))

(event Custom|SetBinaryView
  (params (BinaryView :type Binar%20Experiment%20View%20Object%20Reference))
  (Variables|Default|SetUIBinaryInstruction BinaryView))

(event EventBeginPlay
  (for _array_element (Variables|Default|GetLightbulbs)
    (EventDispatchers|BindEventtoHasBeenTouched _array_element (delegate Custom|CheckIfNumberIsCorrect))
    (Default|ChangeName (Variables|Default|GetBinaryDisplay) "Binär")
    (Default|ChangeName (Variables|Default|GetDecimalDisplay) "Dezimal")))

(event EventOnActivateExperiment
  (bind _uibinaryinstruction (Variables|Default|GetUIBinaryInstruction))
  (|CallParentFunction)
  (Variables|Default|SetisExperimentActive true)
  (CallFunction|SetMaxTouches)
  (CallFunction|GetRandomNumber)
  (Utilities|Array|Clear (Variables|Default|GetUsedRandomNumbers))
  (CallFunction|SwitchOffAllLightbulbs)
  (if (Utilities|IsValid _uibinaryinstruction)
    (UserInterface|Viewport|AddtoViewport _uibinaryinstruction 0)))

(event EventOnDeactivateExperiment
  (|CallParentFunction)
  (Variables|Default|SetRandomNumber 0)
  (Variables|Default|SetNumberOfCorrectAnswers 0)
  (Utilities|Array|Clear (Variables|Default|GetUsedRandomNumbers))
  (CallFunction|SetMaxTouches)
  (Variables|Default|SetisExperimentActive false)
  (Widget|RemovefromParent (Variables|Default|GetUIBinaryInstruction)))

(fn ConstructionScript
  (|CallParentFunction))

(fn CheckforCorrectBinaryNumber
  (for _array_element (Variables|Default|GetLightbulbs)
    (if (Variables|/Game/Blueprints/Experiment2/BP_Lightbulb.BP_Lightbulb_C|GetisLightOn _array_element)
      (LocalVariables|SetSumOfLightbulbNumbers (+ (LocalVariables|GetSumOfLightbulbNumbers) (Math|Float|Power 2.0 (Math|Conversions|ToFloat(Integer) (LocalVariables|GetLightbulbIndex))))))
    (Math|Integer|IncrementInt (LocalVariables|GetLightbulbIndex)))
  (if (== (LocalVariables|GetSumOfLightbulbNumbers) (Variables|Default|GetRandomNumber))
    (return true)
    (else
      (return false))))

(fn SwitchOffAllLightbulbs
  (for _array_element (Variables|Default|GetLightbulbs)
    (Default|SetLight _array_element false)))

(fn SetMaxTouches
  (switch Utilities|FlowControl|Switch|SwitchonExperimentDifficulty (Variables|Default|GetDifficulty)
    (:NewEnumerator0
      (Variables|Default|SetNumberOfMaxTouches (+ (Utilities|Array|Length (Variables|Default|GetLightbulbs)) 2) :!label _label))
    (:NewEnumerator1
      (goto _label))
    (:NewEnumerator2
      (Variables|Default|SetNumberOfMaxTouches (+ (Utilities|Array|Length (Variables|Default|GetLightbulbs)) 1)))))

(fn GetNewRandomNumber
  (switch Utilities|FlowControl|Switch|SwitchonExperimentDifficulty (Variables|Default|GetDifficulty) :!label _label
    (:NewEnumerator0
      (Variables|Default|SetRandomNumber (Math|Random|RandomIntegerinRange 1 15)))
    (:NewEnumerator1
      (Variables|Default|SetRandomNumber (Math|Random|RandomIntegerinRange 1 31)))
    (:NewEnumerator2
      (Variables|Default|SetRandomNumber (Math|Random|RandomIntegerinRange 1 63))))
  (for _array_element (Variables|Default|GetUsedRandomNumbers)
    (if (== _array_element (Variables|Default|GetRandomNumber))
      (LocalVariables|SetisNumberUsedAlready true)))
  (if true
    (goto _label)
    (else
      (Utilities|Array|Add (Variables|Default|GetUsedRandomNumbers) (Variables|Default|GetRandomNumber)))))

(fn GetDecimalNumberfromTorches
  (for _array_element (Variables|Default|GetLightbulbs)
    (if (Variables|/Game/Blueprints/Experiment2/BP_Lightbulb.BP_Lightbulb_C|GetisLightOn _array_element)
      (LocalVariables|SetSumOfLightbulbNumbers (+ (LocalVariables|GetSumOfLightbulbNumbers) (Math|Float|Power 2.0 (Math|Conversions|ToFloat(Integer) (LocalVariables|GetLightbulbIndex))))))
    (Math|Integer|IncrementInt (LocalVariables|GetLightbulbIndex)))
  (return (LocalVariables|GetSumOfLightbulbNumbers)))

(fn GetBinaryNumberfromTorches
  (for _array_element (Variables|Default|GetLightbulbs)
    (if (Variables|/Game/Blueprints/Experiment2/BP_Lightbulb.BP_Lightbulb_C|GetisLightOn _array_element)
      (LocalVariables|SetBinaryNumber (Utilities|String|Append "1" (LocalVariables|GetBinaryNumber)))
      (else
        (LocalVariables|SetBinaryNumber (Utilities|String|Append "0" (LocalVariables|GetBinaryNumber))))))
  (return (Math|Conversions|ToInteger(Byte) (LocalVariables|GetBinaryNumber))))