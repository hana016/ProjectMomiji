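; Game manager that handles the main menu and the transition into gameplay.
; On BeginPlay it deactivates its listed actors through IActivate, hides the player's coin view, shows MainMenu and switches mobile controls after a short delay.
; Pressing Start removes the menu, reactivates the actors and shows coins.
; Player IDs starting with "b" get the Shop disabled as a customization feature, then Logger reads its file and logs the game start.
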(event Custom|StartGame
  (bind _player (Variables|Default|GetPlayer))
  (bind _logger (Variables|Default|GetLogger))
  (Widget|RemovefromParent (Variables|Default|GetMainMenu))
  (CallFunction|ActivateAllActors)
  (Default|EnableCoinView _player true)
  (if (Utilities|Enum|Equal(Enum) (Utilities|String|GetSubstring (Variables|/Game/FirstPerson/Blueprints/BP_FirstPersonCharacter.BP_FirstPersonCharacter_C|GetPlayerID _player) 0) "b")
    (CallFunction|EnableCustomizationFeatures false))
  (Default|ReadLogfromFile _logger)
  (Default|LogGameStart _logger))

(event Custom|ActivateAllActors
  (for _array_element (Variables|Default|GetActorsToActivate)
    (bind _asiactivate (Utilities|Casting|CastToIActivate _array_element))
    (Default|Activate _asiactivate)))

(event Custom|DeactivateAllActors
  (for _array_element (Variables|Default|GetActorsToActivate)
    (bind _asiactivate (Utilities|Casting|CastToIActivate _array_element))
    (Default|Deactivate _asiactivate)))

(event Custom|EnableCustomizationFeatures
  (params (Enable :type Boolean))
  (if (not Enable)
    (Default|DisableShop (Variables|Default|GetShop))))

(event EventBeginPlay
  (CallFunction|DeactivateAllActors)
  (bind _asbp_first_person_character (Utilities|Casting|CastToBP_FirstPersonCharacter (Game|GetPlayerCharacter 0)))
  (bind _output_get (Variables|Default|SetPlayer _asbp_first_person_character))
  (Default|EnableCoinView _output_get false)
  (bind _returnvalue (UserInterface|CreateWidget "/Game/Blueprints/Menus/MainMenu.MainMenu_C"))
  (bind _output_get_2 (Variables|Default|SetMainMenu _returnvalue))
  (Variables|/Game/Blueprints/Menus/MainMenu.MainMenu_C|SetPlayer _output_get_2 (Variables|Default|GetPlayer))
  (EventDispatchers|BindEventtoOnStartPressed _output_get_2 (delegate Custom|StartGame))
  (UserInterface|Viewport|AddtoViewport _output_get_2 0)
  (Utilities|FlowControl|Delay 0.2)
  (Default|SwitchMobileControlls (Variables|Default|GetPlayer) "NewEnumerator2"))

(fn ConstructionScript)