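; BP_Logging records timestamped gameplay events to a per-player text file in the project content directory, named by the first-person character's PlayerID.
; Typed events for game start, tables, experiments, solution attempts and customization menus build semicolon-delimited entries with UTC time and tags.
; All feed WriteLogToFIle, which appends to an in-memory string and saves it whole each time.
; A separate ReadLogFromFile event loads existing contents into that string.
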(event Custom|WriteLogToFIle
  (params (newLogStatement :type String))
  (Variables|Default|SetStringToFIle (Utilities|String|Append (Variables|Default|GetStringToFIle) newLogStatement " 
"))
  (Class|ReadandWriteFileBPLibrary|SaveStringtoFile (Utilities|String|Append (Class|KismetSystemLibrary|GetProjectContentDirectory) "/" (Variables|/Game/FirstPerson/Blueprints/BP_FirstPersonCharacter.BP_FirstPersonCharacter_C|GetPlayerID (Variables|Default|GetPlayer)) ".txt") (Variables|Default|GetStringToFIle)))

(event Custom|ReadLogFromFile
  (bind (_success _infomessage _emptytext _returnvalue) (Class|ReadandWriteFileBPLibrary|ReadStringfromFile (Utilities|String|Append (Class|KismetSystemLibrary|GetProjectContentDirectory) "/" (Variables|/Game/FirstPerson/Blueprints/BP_FirstPersonCharacter.BP_FirstPersonCharacter_C|GetPlayerID (Variables|Default|GetPlayer)) ".txt")))
  (if _success
    (Variables|Default|SetStringToFIle _returnvalue)
    (else
      (Variables|Default|SetStringToFIle ""))))

(event Custom|LogTableStartAndEnd
  (params (Tag :type String) (TableID :type Integer) (ExperimentType :type ExperimentType%20Enum :default "NewEnumerator0"))
  (bind _returnvalue (Math|DateTime|UTCNow))
  (bind (_year _month _day _hour _minute _second _millisecond) (Math|DateTime|BreakDateTime _returnvalue))
  (CallFunction|WriteLogtoFIle (Utilities|String|Append (Utilities|String|Append (Utilities|String|ToString(Integer) _hour) ":" (Utilities|String|ToString(Integer) _minute) ":" (Utilities|String|ToString(Integer) _second) ":" (Utilities|String|ToString(Integer) _millisecond)) ";" Tag ";" (Utilities|String|ToString(Integer) TableID) ";" (Utilities|String|EnumtoString ExperimentType))))

(event Custom|LogExperimentStartAndEnd
  (params (Tag :type String) (TableID :type Integer) (ExperimentType :type ExperimentType%20Enum :default "NewEnumerator0") (ExperimentID :type Integer) (Difficulty :type ExperimentDifficulty%20Enum :default "NewEnumerator0") (Success :type ExperimentOutcome%20Enum :default "NewEnumerator0"))
  (bind _returnvalue (Math|DateTime|UTCNow))
  (bind (_year _month _day _hour _minute _second _millisecond) (Math|DateTime|BreakDateTime _returnvalue))
  (CallFunction|WriteLogtoFIle (Utilities|String|Append (Utilities|String|Append (Utilities|String|ToString(Integer) _hour) ":" (Utilities|String|ToString(Integer) _minute) ":" (Utilities|String|ToString(Integer) _second) ":" (Utilities|String|ToString(Integer) _millisecond)) ";" Tag ";" (Utilities|String|ToString(Integer) TableID) ";" (Utilities|String|EnumtoString ExperimentType) ";" (Utilities|String|ToString(Integer) ExperimentID) ";" (Utilities|String|EnumtoString Difficulty) ";" (Utilities|String|EnumtoString Success))))

(event Custom|LogExperimentSolutionAttempt
  (params (TableID :type Integer) (ExperimentType :type ExperimentType%20Enum :default "NewEnumerator0") (ExperimentID :type Integer) (Difficulty :type ExperimentDifficulty%20Enum :default "NewEnumerator0") (Success :type ExperimentOutcome%20Enum :default "NewEnumerator0"))
  (bind _returnvalue (Math|DateTime|UTCNow))
  (bind (_year _month _day _hour _minute _second _millisecond) (Math|DateTime|BreakDateTime _returnvalue))
  (CallFunction|WriteLogtoFIle (Utilities|String|Append (Utilities|String|Append (Utilities|String|ToString(Integer) _hour) ":" (Utilities|String|ToString(Integer) _minute) ":" (Utilities|String|ToString(Integer) _second) ":" (Utilities|String|ToString(Integer) _millisecond)) ";" "ESA" ";" (Utilities|String|ToString(Integer) TableID) ";" (Utilities|String|EnumtoString ExperimentType) ";" (Utilities|String|ToString(Integer) ExperimentID) ";" (Utilities|String|EnumtoString Difficulty) ";" (Utilities|String|EnumtoString Success))))

(event Custom|LogGameStart
  (bind _returnvalue (Math|DateTime|UTCNow))
  (bind (_year _month _day _hour _minute _second _millisecond) (Math|DateTime|BreakDateTime _returnvalue))
  (CallFunction|WriteLogtoFIle (Utilities|String|Append (Utilities|String|Append (Utilities|String|ToString(Integer) _hour) ":" (Utilities|String|ToString(Integer) _minute) ":" (Utilities|String|ToString(Integer) _second) ":" (Utilities|String|ToString(Integer) _millisecond)) ";" "GS")))

(event Custom|LogCustomizationMenuStartAndEnd
  (params (Tag :type String) (MenuID :type Integer))
  (bind _returnvalue (Math|DateTime|UTCNow))
  (bind (_year _month _day _hour _minute _second _millisecond) (Math|DateTime|BreakDateTime _returnvalue))
  (CallFunction|WriteLogtoFIle (Utilities|String|Append (Utilities|String|Append (Utilities|String|ToString(Integer) _hour) ":" (Utilities|String|ToString(Integer) _minute) ":" (Utilities|String|ToString(Integer) _second) ":" (Utilities|String|ToString(Integer) _millisecond)) ";" Tag ";" (Utilities|String|ToString(Integer) MenuID))))

(event Custom|LogCustomizationMenuBought
  (params (MenuID :type Integer) (BodyPart :type CompanionBodyPart%20Enum :default "NewEnumerator0") (Difficulty :type ExperimentDifficulty%20Enum :default "NewEnumerator0") (ItemName :type String) (isUnlocked :type Boolean))
  (bind _returnvalue (Math|DateTime|UTCNow))
  (bind (_year _month _day _hour _minute _second _millisecond) (Math|DateTime|BreakDateTime _returnvalue))
  (if isUnlocked
    (Variables|Default|SetUnlockedString "Unlocked")
    (else
      (Variables|Default|SetUnlockedString "Locked")))
  (CallFunction|WriteLogtoFIle (Utilities|String|Append (Utilities|String|Append (Utilities|String|ToString(Integer) _hour) ":" (Utilities|String|ToString(Integer) _minute) ":" (Utilities|String|ToString(Integer) _second) ":" (Utilities|String|ToString(Integer) _millisecond)) ";" "CMB" ";" (Utilities|String|ToString(Integer) MenuID) ";" (Utilities|String|EnumtoString BodyPart) ";" (Utilities|String|EnumtoString Difficulty) ";" ItemName ";" (Variables|Default|GetUnlockedString))))

(event EventBeginPlay
  (bind _asbp_first_person_character (Utilities|Casting|CastToBP_FirstPersonCharacter (Game|GetPlayerCharacter 0)))
  (Variables|Default|SetPlayer _asbp_first_person_character))

(fn ConstructionScript)