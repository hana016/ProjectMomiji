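; BP_Shop is a world shop station where the player opens a companion outfit customization menu, shown as a slowly spinning companion mesh.
; Box overlap shows or hides an interact billboard, and interacting lazily creates the ShopMenu widget and switches the player's mobile controls.
; Cancelling resets the companion's outfit, closes the menu, restores controls and logs the session under an incrementing ID.
; DisableShop deactivates the station and hides its meshes.
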(event OnComponentBeginOverlap(Box)
  (params (OverlappedComponent :type Primitive%20Component%20Object%20Reference) (OtherActor :type Actor%20Object%20Reference) (OtherComp :type Primitive%20Component%20Object%20Reference) (OtherBodyIndex :type Integer) (bFromSweep :type Boolean) (SweepResult :type Hit%20Result%20Structure%20%28by%20ref%29))
  (if (Variables|Default|GetisActive)
    (if (Utilities|IsValid (Variables|Default|GetInteractWidget))
      _
      (else
        (bind _returnvalue (UserInterface|CreateWidget "/Game/Blueprints/InteractBillboard.InteractBillboard_C"))
        (bind _output_get (Variables|Default|SetInteractWidget _returnvalue))))
    (UserInterface|Viewport|AddtoViewport _output_get 0)))

(event OnComponentEndOverlap(Box)
  (params (OverlappedComponent :type Primitive%20Component%20Object%20Reference) (OtherActor :type Actor%20Object%20Reference) (OtherComp :type Primitive%20Component%20Object%20Reference) (OtherBodyIndex :type Integer))
  (if (Variables|Default|GetisActive)
    (if (Utilities|IsValid (Variables|Default|GetInteractWidget))
      _
      (else
        (bind _returnvalue (UserInterface|CreateWidget "/Game/Blueprints/InteractBillboard.InteractBillboard_C"))
        (bind _output_get (Variables|Default|SetInteractWidget _returnvalue))))
    (Widget|RemovefromParent _output_get)))

(event Custom|DisableShop
  (Variables|Default|SetisActive false)
  (Rendering|SetVisibility (Variables|Default|Getfbx_CompanionNoSkeleton) false false)
  (Rendering|SetVisibility (Variables|Default|GetCylinder) false false))

(event EventCancelInteracation
  (bind _shopwidget (Variables|Default|GetShopWidget))
  (Default|ResetOutfit (Variables|Default|GetCompanion))
  (Widget|RemovefromParent _shopwidget)
  (Default|OnBackButtonPressed _shopwidget)
  (Default|SwitchMobileControlls (Variables|Default|GetPlayer) "NewEnumerator0")
  (Default|LogCustomizationMenuStartandEnd (Variables|Default|GetLogger) "CME" (Variables|Default|GetSessionID))
  (Math|Integer|IncrementInt (Variables|Default|GetSessionID)))

(event EventButtonInteract
  (if (Variables|Default|GetisActive)
    (if (Utilities|IsValid (Variables|Default|GetShopWidget))
      _
      (else
        (bind _returnvalue (UserInterface|CreateWidget "/Game/Blueprints/Menus/ShopMenu.ShopMenu_C" 0 (Variables|Default|GetCompanion)))
        (Variables|Default|SetShopWidget _returnvalue)))
    (UserInterface|Viewport|AddtoViewport (Variables|Default|GetShopWidget) 0)
    (Default|SwitchMobileControlls (Variables|Default|GetPlayer) "NewEnumerator3")
    (Default|LogCustomizationMenuStartandEnd (Variables|Default|GetLogger) "CMS" (Variables|Default|GetSessionID))))

(event EventTick
  (params (DeltaSeconds :type Float%20%28single-precision%29))
  (bind _fbx_companionnoskeleton (Variables|Default|Getfbx_CompanionNoSkeleton))
  (bind _relativerotation (Variables|/Script/Engine.SceneComponent|GetRelativeRotation _fbx_companionnoskeleton))
  (if (Variables|Default|GetisActive)
    (Transformation|SetRelativeRotation _fbx_companionnoskeleton (Math|Rotator|MakeRotator (.roll _relativerotation) (.pitch _relativerotation) (+ (.yaw _relativerotation) 0.8)) false false)))

(event EventBeginPlay
  (bind _asbp_first_person_character (Utilities|Casting|CastToBP_FirstPersonCharacter (Game|GetPlayerCharacter 0)))
  (Variables|Default|SetPlayer _asbp_first_person_character))

(fn ConstructionScript)