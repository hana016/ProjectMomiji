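; BP_FrequencySlider is an interactive vertical frequency slider for Experiment3, dragged by touch or mouse.
; The first grab caches the button's screen position as the origin, which persists until a reset.
; Touch moves, or mouse position polled on Tick while grabbed, turn the screen Y offset into a clamped local Z position.
; Dispatchers broadcast that value and signal release, while resetting recenters the button and broadcasts zero.
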(event Custom|ResetSliderPosition
  (Variables|Default|SetDefaultButtonLocation "0, 0, 0")
  (Transformation|SetRelativeLocation (Variables|Default|Getfbx_FrequencySliderButton) "0, 0, 0" false false)
  (Default|CallOnSliderChanged 0.0))

(event EventMouseTouch
  (bind _returnvalue (Game|GetPlayerController 0))
  (bind _fbx_frequencysliderbutton (Variables|Default|Getfbx_FrequencySliderButton))
  (bind _returnvalue_2 (Transformation|GetWorldLocation _fbx_frequencysliderbutton))
  (bind _screenposition (Class|GameplayStatics|ProjectWorldtoScreen _returnvalue _returnvalue_2 false))
  (Variables|Default|SetisSliderGrabbed true)
  (if (== (.y (Variables|Default|GetDefaultButtonLocation)) 0.0)
    (Variables|Default|SetDefaultButtonLocation (Math|Vector|MakeVector (.x _screenposition) (.y _screenposition) 1.0))))

(event EventBeginPlay)

(event EventMouseTouchRelease
  (Variables|Default|SetisSliderGrabbed false)
  (Default|CallOnSliderReleased))

(event EventTick
  (params (DeltaSeconds :type Float%20%28single-precision%29))
  (bind _returnvalue (Game|GetPlayerController 0))
  (bind _defaultbuttonlocation (Variables|Default|GetDefaultButtonLocation))
  (bind (_locationx _locationy) (Game|Player|GetMousePosition _returnvalue))
  (bind _returnvalue_2 (- (Math|Vector|MakeVector _locationx _locationy 0.0) _defaultbuttonlocation))
  (bind _returnvalue_3 (/ (.y _returnvalue_2) 15.0))
  (bind _returnvalue_4 (* _returnvalue_3 -1.0))
  (bind _returnvalue_5 (Math|Float|Clamp(Float) _returnvalue_4 -9.0 9.0))
  (if (Variables|Default|GetisSliderGrabbed)
    (Transformation|SetRelativeLocation (Variables|Default|Getfbx_FrequencySliderButton) (Math|Vector|MakeVector 0.0 0.0 _returnvalue_5) false false)
    (Default|CallOnSliderChanged _returnvalue_5)))

(event EventTouchMoveInteract
  (params (Location :type Vector :default "0, 0, 0"))
  (bind _defaultbuttonlocation (Variables|Default|GetDefaultButtonLocation))
  (bind _returnvalue (- Location _defaultbuttonlocation))
  (bind _returnvalue_2 (/ (.y _returnvalue) 15.0))
  (bind _returnvalue_3 (* _returnvalue_2 -1.0))
  (bind _returnvalue_4 (Math|Float|Clamp(Float) _returnvalue_3 -9.0 9.0))
  (Variables|Default|SetisSliderGrabbed true)
  (Transformation|SetRelativeLocation (Variables|Default|Getfbx_FrequencySliderButton) (Math|Vector|MakeVector 0.0 0.0 _returnvalue_4) false false)
  (Default|CallOnSliderChanged _returnvalue_4))

(event EventTouchRelease
  (Variables|Default|SetisSliderGrabbed false)
  (Default|CallOnSliderReleased))

(event EventTouchInteract
  (params (Location :type Vector :default "0, 0, 0"))
  (bind _returnvalue (Game|GetPlayerController 0))
  (bind _fbx_frequencysliderbutton (Variables|Default|Getfbx_FrequencySliderButton))
  (bind _returnvalue_2 (Transformation|GetWorldLocation _fbx_frequencysliderbutton))
  (bind _screenposition (Class|GameplayStatics|ProjectWorldtoScreen _returnvalue _returnvalue_2 false))
  (Variables|Default|SetisSliderGrabbed true)
  (if (== (.y (Variables|Default|GetDefaultButtonLocation)) 0.0)
    (Variables|Default|SetDefaultButtonLocation (Math|Vector|MakeVector (.x _screenposition) (.y _screenposition) 1.0))))

(fn ConstructionScript)