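; Touch-operated frequency wheel on a stand for Experiment 3, which the player turns by dragging a finger around it.
; A helper projects the stand to screen space and derives the finger's angle with acos, using a vertical dot-product test to choose the mirrored half for full-circle roll.
; Moves and resets broadcast RotationChanged, release broadcasts WheelReleased, and the initial touch only rotates the wheel and marks it grabbed.
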(event Custom|ResetWheelRotation
  (Transformation|SetRelativeRotation (Variables|Default|Getfbx_Frequency_wheel) "0, 0, 0" false false)
  (Default|CallRotationChanged 0.0))

(event EventTouchMoveInteract
  (params (Location :type Vector :default "0, 0, 0"))
  (Variables|Default|SetisWheelGrabbed true)
  (bind (_returnvalue _returnvalue2 _returnvalue3) (CallFunction|CalculateWheelRotationAccordingtoFingerLocation Location))
  (if _returnvalue2
    (Transformation|SetRelativeRotation (Variables|Default|Getfbx_Frequency_wheel) (Math|Rotator|MakeRotator _returnvalue 0.0 0.0) false false)
    (Default|CallRotationChanged (.roll (Variables|/Script/Engine.SceneComponent|GetRelativeRotation (Variables|Default|Getfbx_Frequency_wheel))))
    (else
      (Transformation|SetRelativeRotation (Variables|Default|Getfbx_Frequency_wheel) (Math|Rotator|MakeRotator _returnvalue3 0.0 0.0) false false)
      (Default|CallRotationChanged (.roll (Variables|/Script/Engine.SceneComponent|GetRelativeRotation (Variables|Default|Getfbx_Frequency_wheel)))))))

(event EventTouchInteract
  (params (Location :type Vector :default "0, 0, 0"))
  (Variables|Default|SetisWheelGrabbed true)
  (bind (_returnvalue _returnvalue2 _returnvalue3) (CallFunction|CalculateWheelRotationAccordingtoFingerLocation Location))
  (if _returnvalue2
    (Transformation|SetRelativeRotation (Variables|Default|Getfbx_Frequency_wheel) (Math|Rotator|MakeRotator _returnvalue 0.0 0.0) false false)
    (else
      (Transformation|SetRelativeRotation (Variables|Default|Getfbx_Frequency_wheel) (Math|Rotator|MakeRotator _returnvalue3 0.0 0.0) false false))))

(event EventTouchRelease
  (Variables|Default|SetisWheelGrabbed false)
  (Default|CallWheelReleased))

(fn ConstructionScript)

(fn CalculateWheelRotationAccordingtoFingerLocation
  (params (Location :type Vector))
  (bind _returnvalue (Game|GetPlayerController 0))
  (bind _returnvalue_2 (Class|KismetMathLibrary|VectorNormal2D "-1.000000,0.000000,1.000000" 0.0001))
  (bind _fbx_frequency_wheelstand (Variables|Default|Getfbx_Frequency_wheelStand))
  (bind _returnvalue_3 (Transformation|GetWorldLocation _fbx_frequency_wheelstand))
  (bind _screenposition (Class|GameplayStatics|ProjectWorldtoScreen _returnvalue _returnvalue_3 false))
  (bind _returnvalue_4 (- Location _screenposition))
  (bind _returnvalue_5 (Class|KismetMathLibrary|VectorNormal2D _returnvalue_4 0.0001))
  (bind _returnvalue_6 (Math|Vector|DotProduct _returnvalue_2 _returnvalue_5))
  (bind _returnvalue_7 (Class|KismetMathLibrary|DegAcos _returnvalue_6))
  (return (+ (+ (- 1.8e+02 _returnvalue_7) 1.8e+02) 9e+01) (> (Math|Trig|Sin(Degrees) (Math|Vector|DotProduct (Class|KismetMathLibrary|VectorNormal2D "0.000000,-1.000000,1.000000" 0.0001) _returnvalue_5)) 0.0) (+ _returnvalue_7 9e+01)))