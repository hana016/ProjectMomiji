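; Sine-wave puzzle experiment where sliders set amplitude, frequency and phase shift to fit a curve through randomly spawned hit points.
; Tick spawns light particles that trace the player's sine curve, while widgets and an optional violin sound follow the values.
; Difficulty decides how many curve parameters are randomized.
; Releasing a slider compares both curves at each hit point within a tolerance, starting new rounds until enough are solved.
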(event Custom|OnFrequencyChanged
  (params (SliderPosition :type Float%20%28double-precision%29))
  (if (Variables|Default|GetisExperimentActive)
    (Variables|Default|SetFrequency (/ SliderPosition 2.0))
    (CallFunction|SetSoundFrequencyandAmplitude)
    (CallFunction|ChangeWidgetValues)))

(event Custom|SetMusic
  (params (MusicOn :type Boolean))
  (bind _isexperimentactive (Variables|Default|GetisExperimentActive))
  (Variables|Default|SetisMusicOn MusicOn)
  (if _isexperimentactive
    (if (and _isexperimentactive MusicOn)
      (if (Utilities|IsValid (Variables|Default|GetSoundWave))
        _
        (else
          (bind _returnvalue (Audio|CreateSound2D "/Game/Sounds/ViolinFrequencyAndAmplitudeChangable.ViolinFrequencyAndAmplitudeChangable" 1.0 1.0 0.0 0))
          (Variables|Default|SetSoundWave _returnvalue)))
      (CallFunction|SetSoundFrequencyandAmplitude)
      (Audio|Components|Audio|Play (Variables|Default|GetSoundWave) 0.0)
      (else
        (Audio|Components|Audio|Stop (Variables|Default|GetSoundWave))))))

(event Custom|SetFrequencyView
  (params (FrequencyView :type Frequency%20Experiment%20View%20Object%20Reference))
  (Variables|Default|SetFrequencyExperimentView FrequencyView))

(event Custom|SpawnNewRandomHitPoints
  (CallFunction|ResetAllVariables)
  (CallFunction|SetSoundFrequencyandAmplitude)
  (CallFunction|SetMusic (Variables|Default|GetisMusicOn))
  (CallFunction|ChangeWidgetValues)
  (CallFunction|SetRandomCurveVariables)
  (switch Utilities|FlowControl|Switch|SwitchonExperimentDifficulty (Variables|Default|GetDifficulty)
    (:NewEnumerator0
      (for _index (range 0 3)
        (bind _y (CallFunction|CalculateFrequenceFunction (Variables|Default|GetAmplitude) (Variables|Default|GetRandom%20Frequency) (Variables|Default|GetRandomTime) (Variables|Default|GetPhaseShift)))
        (CallFunction|SpawnHitPoint (Variables|Default|GetRandomTime) _y)
        (Variables|Default|SetRandomAmplitude (Variables|Default|GetAmplitude))
        (Variables|Default|SetRandomPhaseShift (Variables|Default|GetPhaseShift))
        (Variables|Default|SetRandomTime (Math|Float|Clamp(Float) (+ (Variables|Default|GetRandomTime) (Math|Random|RandomFloatinRange -5.0 -2e+01)) -6e+01 -1.0))))
    (:NewEnumerator1
      (for _index_2 (range 0 3)
        (bind _y_2 (CallFunction|CalculateFrequenceFunction (Variables|Default|GetRandomAmplitude) (Variables|Default|GetRandom%20Frequency) (Variables|Default|GetRandomTime) (Variables|Default|GetPhaseShift)))
        (CallFunction|SpawnHitPoint (Variables|Default|GetRandomTime) _y_2)
        (Variables|Default|SetRandomPhaseShift (Variables|Default|GetPhaseShift))
        (Variables|Default|SetRandomTime (Math|Float|Clamp(Float) (+ (Variables|Default|GetRandomTime) (Math|Random|RandomFloatinRange -5.0 -2e+01)) -6e+01 -1.0))))
    (:NewEnumerator2
      (for _index_3 (range 0 3)
        (bind _y_3 (CallFunction|CalculateFrequenceFunction (Variables|Default|GetRandomAmplitude) (Variables|Default|GetRandom%20Frequency) (Variables|Default|GetRandomTime) (Variables|Default|GetRandomPhaseShift)))
        (CallFunction|SpawnHitPoint (Variables|Default|GetRandomTime) _y_3)
        (Variables|Default|SetRandomTime (Math|Float|Clamp(Float) (+ (Variables|Default|GetRandomTime) (Math|Random|RandomFloatinRange -5.0 -2e+01)) -6e+01 -1.0))))))

(event Custom|OnChangeAmplitude
  (params (SliderPosition :type Float%20%28double-precision%29))
  (if (Variables|Default|GetisExperimentActive)
    (Variables|Default|SetAmplitude (Math|Float|Absolute(Float) SliderPosition))
    (CallFunction|SetSoundFrequencyandAmplitude)
    (CallFunction|ChangeWidgetValues)))

(event Custom|OnWheelReleased
  (if (Variables|Default|GetisExperimentActive)
    (bind _allhitpointshit (CallFunction|CheckifAllHitpointsHit))
    (if _allhitpointshit
      (Math|Integer|IncrementInt (Variables|Default|GetNumberOfCorrectAnswers)
        (:%20%20
          (if (< (Variables|Default|GetNumberOfCorrectAnswers) (Variables|Default|GetNumberOfNeededCorrectAnswers))
            (Audio|PlaySound2D "/Game/Sounds/Plopp.Plopp" 1.0 1.0 0.0 0 0)
            (CallFunction|SpawnNewRandomHitPoints)
            (else
              (Variables|Default|SetspawnParticles false)
              (Audio|PlaySound2D "/Game/Sounds/Plopp.Plopp" 1.0 1.0 0.0 0 0)
              (CallFunction|FinishSuccessfully))))))))

(event Custom|OnPhaseShiftChanged
  (params (SliderPosition :type Float%20%28double-precision%29))
  (if (Variables|Default|GetisExperimentActive)
    (Variables|Default|SetPhaseShift (* SliderPosition 1e+01))
    (CallFunction|ChangeWidgetValues)))

(event EventTick
  (params (DeltaSeconds :type Float%20%28single-precision%29))
  (Utilities|FlowControl|Delay 0.01)
  (if (Variables|Default|GetisExperimentActive)
    (CallFunction|SetParticleYCoordinates)
    (if (and (< (Utilities|Array|Length (Variables|Default|GetLightparticles)) 201) (Variables|Default|GetspawnParticles))
      (bind _returnvalue (Game|SpawnActorfromClass "/Game/Blueprints/Experiment3/BP_Lightparticle.BP_Lightparticle_C" (Variables|Default|GetSpawnLocation) "AlwaysSpawn" "MultiplyWithRoot" 0 0))
      (Utilities|Array|Add (Variables|Default|GetLightparticles) _returnvalue))))

(event EventBeginPlay
  (bind _fbx_frequency (Variables|Default|Getfbx_Frequency))
  (bind _frequencyslider (Variables|Default|GetFrequencySlider))
  (bind _amplitudeslider (Variables|Default|GetAmplitudeSlider))
  (bind _phaseshiftslider (Variables|Default|GetPhaseShiftSlider))
  (bind _returnvalue (Transformation|GetWorldTransform _fbx_frequency))
  (Variables|Default|SetSpawnLocation (Math|Transform|MakeTransform (Math|Vector|MakeVector (.x (.location _returnvalue)) (.y (.location _returnvalue)) (+ (.z (.location _returnvalue)) 15.0)) (.rotation _returnvalue) "1.000000,1.000000,1.000000"))
  (if (Utilities|IsValid (Variables|Default|GetAmplitudeSlider))
    (EventDispatchers|BindEventtoOnSliderChanged _amplitudeslider (delegate Custom|OnChangeAmplitude))
    (EventDispatchers|BindEventtoOnSliderReleased _amplitudeslider (delegate Custom|OnWheelReleased)))
  (if (Utilities|IsValid (Variables|Default|GetFrequencySlider))
    (EventDispatchers|BindEventtoOnSliderChanged _frequencyslider (delegate Custom|OnFrequencyChanged))
    (EventDispatchers|BindEventtoOnSliderReleased _frequencyslider (delegate Custom|OnWheelReleased)))
  (if (Utilities|IsValid (Variables|Default|GetPhaseShiftSlider))
    (EventDispatchers|BindEventtoOnSliderChanged _phaseshiftslider (delegate Custom|OnPhaseShiftChanged))
    (EventDispatchers|BindEventtoOnSliderReleased _phaseshiftslider (delegate Custom|OnWheelReleased))))

(event EventOnDeactivateExperiment
  (|CallParentFunction)
  (CallFunction|ResetAllVariables)
  (Widget|RemovefromParent (Variables|Default|GetFrequencyExperimentView))
  (Variables|Default|SetNumberOfCorrectAnswers 0)
  (Audio|Components|Audio|Stop (Variables|Default|GetSoundWave)))

(event EventOnActivateExperiment
  (|CallParentFunction)
  (CallFunction|ResetAllVariables)
  (if (Utilities|IsValid (Variables|Default|GetFrequencyExperimentView))
    (UserInterface|Viewport|AddtoViewport (Variables|Default|GetFrequencyExperimentView) 0))
  (Variables|Default|SetNumberOfCorrectAnswers 0)
  (CallFunction|SpawnNewRandomHitPoints)
  (Variables|Default|SetspawnParticles true))

(fn ConstructionScript)

(fn CalculateFrequenceFunction
  (params (Amplitude :type Float%20%28double-precision%29) (Frequency :type Float%20%28double-precision%29) (t :type Float%20%28double-precision%29) (PhaseShift :type Float%20%28double-precision%29))
  (return (* Amplitude (Math|Trig|Sin(Degrees) (+ (* (* Frequency (Math|Float|MultiplybyPi 2.0)) t) PhaseShift)))))

(fn SetParticleYCoordinates
  (for _array_element (Variables|Default|GetLightparticles)
    (if (< (.y (.location (Transformation|GetRelativeTransform (Variables|/Game/Blueprints/Experiment3/BP_Lightparticle.BP_Lightparticle_C|Getparticle _array_element)))) -6e+01)
      ;[1 1 1] If Particles Reach the end, reset them to 0
      (Transformation|SetRelativeLocation (Variables|/Game/Blueprints/Experiment3/BP_Lightparticle.BP_Lightparticle_C|Getparticle _array_element) (Math|Vector|MakeVector (.x (.location (Transformation|GetRelativeTransform (Variables|/Game/Blueprints/Experiment3/BP_Lightparticle.BP_Lightparticle_C|Getparticle _array_element)))) 0.0 (.z (.location (Transformation|GetRelativeTransform (Variables|/Game/Blueprints/Experiment3/BP_Lightparticle.BP_Lightparticle_C|Getparticle _array_element))))) false false)
      (bind _y (CallFunction|CalculateFrequenceFunction (Variables|Default|GetAmplitude) (Variables|Default|GetFrequency) (+ (.y (.location (Transformation|GetRelativeTransform (Variables|/Game/Blueprints/Experiment3/BP_Lightparticle.BP_Lightparticle_C|Getparticle _array_element)))) -0.3) (Variables|Default|GetPhaseShift)))
      (Transformation|SetRelativeLocation (Variables|/Game/Blueprints/Experiment3/BP_Lightparticle.BP_Lightparticle_C|Getparticle _array_element) (Math|Vector|MakeVector (.x (.location (Transformation|GetRelativeTransform (Variables|/Game/Blueprints/Experiment3/BP_Lightparticle.BP_Lightparticle_C|Getparticle _array_element)))) (+ (.y (.location (Transformation|GetRelativeTransform (Variables|/Game/Blueprints/Experiment3/BP_Lightparticle.BP_Lightparticle_C|Getparticle _array_element)))) -0.3) _y) false false)
      (else
        (bind _y_2 (CallFunction|CalculateFrequenceFunction (Variables|Default|GetAmplitude) (Variables|Default|GetFrequency) (+ (.y (.location (Transformation|GetRelativeTransform (Variables|/Game/Blueprints/Experiment3/BP_Lightparticle.BP_Lightparticle_C|Getparticle _array_element)))) -0.3) (Variables|Default|GetPhaseShift)))
        (Transformation|SetRelativeLocation (Variables|/Game/Blueprints/Experiment3/BP_Lightparticle.BP_Lightparticle_C|Getparticle _array_element) (Math|Vector|MakeVector (.x (.location (Transformation|GetRelativeTransform (Variables|/Game/Blueprints/Experiment3/BP_Lightparticle.BP_Lightparticle_C|Getparticle _array_element)))) (+ (.y (.location (Transformation|GetRelativeTransform (Variables|/Game/Blueprints/Experiment3/BP_Lightparticle.BP_Lightparticle_C|Getparticle _array_element)))) -0.3) _y_2) false false)))))

(fn NormalizeRotationinRange
  (params (Rotation :type Float%20%28double-precision%29) (Min :type Float%20%28double-precision%29) (Max :type Float%20%28double-precision%29))
  (return (* Rotation (/ Max 1.8e+02))))

(fn SpawnHitPoint
  (params (Width :type Float%20%28double-precision%29) (Height :type Float%20%28double-precision%29))
  (bind _spawnlocation (Variables|Default|GetSpawnLocation))
  (bind _output_get (LocalVariables|SetRelativeSpawnTransform (Math|Transform|MakeTransform (Math|Vector|MakeVector (.x (.location _spawnlocation)) (+ (.y (.location _spawnlocation)) Width) (+ (.z (.location _spawnlocation)) Height)) (.rotation _spawnlocation) (.scale _spawnlocation))))
  (bind _returnvalue (Game|SpawnActorfromClass "/Game/Blueprints/Experiment3/BP_FrequencyHitPoint.BP_FrequencyHitPoint_C" _output_get "AlwaysSpawn" "MultiplyWithRoot" 0 0))
  (Utilities|Array|Add (Variables|Default|GetHitPoints) _returnvalue))

(fn ResetAllVariables
  (bind _hitpoints (Variables|Default|GetHitPoints))
  (bind _lightparticles (Variables|Default|GetLightparticles))
  (Variables|Default|SetRandom%20Frequency 0.1)
  (Variables|Default|SetRandomAmplitude 9.0)
  (Variables|Default|SetRandomPhaseShift 0.0)
  (Variables|Default|SetAmplitude 9.0)
  (Variables|Default|SetFrequency 0.1)
  (Variables|Default|SetPhaseShift 0.0)
  (for _array_element _hitpoints
    (Actor|DestroyActor _array_element))
  (Utilities|Array|Clear _hitpoints)
  (for _array_element_2 _lightparticles
    (Actor|DestroyActor _array_element_2))
  (Utilities|Array|Clear _lightparticles)
  (Default|ResetSliderPosition (Variables|Default|GetFrequencySlider))
  (if (Utilities|IsValid (Variables|Default|GetAmplitudeSlider))
    (Default|ResetSliderPosition (Variables|Default|GetAmplitudeSlider)))
  (if (Utilities|IsValid (Variables|Default|GetPhaseShiftSlider))
    (Default|ResetSliderPosition (Variables|Default|GetPhaseShiftSlider)))
  (Variables|Default|SetallHitPointsHit true)
  (bind _asdisplay_value (Utilities|Casting|CastToDisplayValue (UserInterface|GetWidget (Variables|Default|GetWidgetFrequency))))
  (Default|ChangeValue _asdisplay_value 0.0)
  (bind _asdisplay_value_2 (Utilities|Casting|CastToDisplayValue (UserInterface|GetWidget (Variables|Default|GetWidgetAmplitude))))
  (Default|ChangeValue _asdisplay_value_2 0.0)
  (bind _asdisplay_value_3 (Utilities|Casting|CastToDisplayValue (UserInterface|GetWidget (Variables|Default|GetWidgetPhaseShift))))
  (Default|ChangeValue _asdisplay_value_3 0.0)
  (CallFunction|SetSoundFrequencyandAmplitude))

(fn CheckifAllHitpointsHit
  (LocalVariables|SetAreAllHitpointsHit true)
  (for _array_element (Variables|Default|GetHitPoints)
    (bind _y (CallFunction|CalculateFrequenceFunction (Variables|Default|GetRandomAmplitude) (Variables|Default|GetRandom%20Frequency) (- (.y (.location (Transformation|GetActorTransform _array_element))) (.y (.location (Variables|Default|GetSpawnLocation)))) (Variables|Default|GetRandomPhaseShift)))
    (LocalVariables|SetSeekedYValue _y)
    (bind _y_2 (CallFunction|CalculateFrequenceFunction (Variables|Default|GetAmplitude) (Variables|Default|GetFrequency) (- (.y (.location (Transformation|GetActorTransform _array_element))) (.y (.location (Variables|Default|GetSpawnLocation)))) (Variables|Default|GetPhaseShift)))
    (LocalVariables|SetSetYValue _y_2)
    (if (not (and (< (- (LocalVariables|GetSeekedYValue) 2.0) (LocalVariables|GetSetYValue)) (< (LocalVariables|GetSetYValue) (+ (LocalVariables|GetSeekedYValue) 2.0))))
      (LocalVariables|SetAreAllHitpointsHit false)))
  (return (LocalVariables|GetAreAllHitpointsHit)))

(fn SetRandomCurveVariables
  (Variables|Default|SetRandom%20Frequency (Math|Random|RandomFloatinRange 1.0 4.0))
  (if (== (Math|Random|RandomIntegerinRange 0 1) 0)
    (Variables|Default|SetRandom%20Frequency (* (Variables|Default|GetRandom%20Frequency) -1.0)))
  (Variables|Default|SetRandomTime -3.0)
  (Variables|Default|SetRandomAmplitude (Math|Random|RandomFloatinRange 3.0 9.0))
  (Variables|Default|SetRandomPhaseShift (Math|Random|RandomFloatinRange 2e+01 9e+01))
  (if (== (Math|Random|RandomIntegerinRange 0 1) 0)
    (Variables|Default|SetRandomPhaseShift (* (Variables|Default|GetRandomPhaseShift) -1.0))))

(fn SetSoundFrequencyandAmplitude
  (bind _soundwave (Variables|Default|GetSoundWave))
  (bind _frequency (Variables|Default|GetFrequency))
  (Audio|Parameter|SetFloatParameter _soundwave "Amplitude" (Math|Float|Clamp(Float) (/ (Variables|Default|GetAmplitude) 1.5) 0.1 9.0) :!class /Script/Engine.AudioComponent)
  (if (< _frequency 0.0)
    (Audio|Parameter|SetFloatParameter _soundwave "Frequency" (Math|Float|Clamp(Float) _frequency -4.5 -1.0) :!class /Script/AudioExtensions.AudioParameterControllerInterface)
    (else
      (Audio|Parameter|SetFloatParameter _soundwave "Frequency" (Math|Float|Clamp(Float) _frequency 0.1 4.5) :!class /Script/AudioExtensions.AudioParameterControllerInterface))))

(fn ChangeWidgetValues
  (bind _asdisplay_value (Utilities|Casting|CastToDisplayValue (UserInterface|GetWidget (Variables|Default|GetWidgetAmplitude))))
  (Default|ChangeValue _asdisplay_value (Variables|Default|GetAmplitude))
  (bind _asdisplay_value_2 (Utilities|Casting|CastToDisplayValue (UserInterface|GetWidget (Variables|Default|GetWidgetFrequency))))
  (Default|ChangeValue _asdisplay_value_2 (Variables|Default|GetFrequency))
  (bind _asdisplay_value_3 (Utilities|Casting|CastToDisplayValue (UserInterface|GetWidget (Variables|Default|GetWidgetPhaseShift))))
  (Default|ChangeValue _asdisplay_value_3 (Variables|Default|GetPhaseShift)))