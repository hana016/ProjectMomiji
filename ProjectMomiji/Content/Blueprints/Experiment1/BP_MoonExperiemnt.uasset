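; Moon phase experiment actor in which the player drags the moon around the Earth by touch or mouse to match a shown phase.
; Drag position becomes moon roll via the angle around Earth's projected screen position; the moon spins idly while inactive.
; Activation shuffles difficulty-filtered phases for the instruction UI.
; Button or auto-check on release tests roll within a tolerance, special-casing full moon's wraparound, logs attempts, then advances or finishes.
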(event Custom|SetNewMoonPhase
  (if (< (Variables|Default|GetCurrentMoonPhaseIndex) (Variables|Default|GetNumberOfNeededCorrectAnswers))
    (Variables|Default|SetCurrentMoonPhase (Utilities|Array|Get(acopy) (Variables|Default|GetMoonPhasesForCurrentDifficulty) (Variables|Default|GetCurrentMoonPhaseIndex)))
    (Variables|Default|SetCurrentMoonPhaseIndex (+ (Variables|Default|GetCurrentMoonPhaseIndex) 1))
    (Default|SetMoonPhaseTexture (Variables|Default|GetUIMoonPhaseInstruction) (.Texture (Utilities|Struct|BreakMoonPhase (Variables|Default|GetCurrentMoonPhase))))
    (else
      (CallFunction|FinishSuccessfully))))

(event Custom|CheckForCorrectMoonPosition
  (bind _table (Variables|Default|GetTable))
  (bind _fbx_moon (Variables|Default|Getfbx_Moon))
  (bind _currentmoonphase (Variables|Default|GetCurrentMoonPhase))
  (bind _table_2 (Variables|Default|GetTable))
  (bind _table_3 (Variables|Default|GetTable))
  (bind _correctposition (Utilities|Struct|BreakMoonPhase _currentmoonphase))
  (bind _relativerotation (Variables|/Script/Engine.SceneComponent|GetRelativeRotation _fbx_moon))
  (if (Utilities|Enum|Equal(Enum) "Vollmond" (.MoonPhaseName (Utilities|Struct|BreakMoonPhase (Variables|Default|GetCurrentMoonPhase))))
    (if (or (and (> (.roll _relativerotation) -181.0) (< (.roll _relativerotation) -1.7e+02)) (and (> (.roll _relativerotation) 1.7e+02) (< (.roll _relativerotation) 181.0)))
      (Audio|PlaySound2D "/Game/Sounds/Plopp.Plopp" 1.0 1.0 0.0 0 0 :!label _label)
      (Default|LogExperimentSolutionAttempt (Variables|Default|GetLogger) (Variables|/Game/Blueprints/BP_ExperimentDesk.BP_ExperimentDesk_C|GetSessionID _table_3) "NewEnumerator0" (Variables|/Game/Blueprints/BP_ExperimentDesk.BP_ExperimentDesk_C|GetExperimentID _table_3) (Variables|/Game/Blueprints/BP_ExperimentDesk.BP_ExperimentDesk_C|GetChosenDifficulty _table_3) "NewEnumerator0")
      (CallFunction|SetNewMoonPhase)
      (else
        (Default|LogExperimentSolutionAttempt (Variables|Default|GetLogger) (Variables|/Game/Blueprints/BP_ExperimentDesk.BP_ExperimentDesk_C|GetSessionID _table_2) "NewEnumerator0" (Variables|/Game/Blueprints/BP_ExperimentDesk.BP_ExperimentDesk_C|GetExperimentID _table_2) (Variables|/Game/Blueprints/BP_ExperimentDesk.BP_ExperimentDesk_C|GetChosenDifficulty _table_2) "NewEnumerator1")
        (CallFunction|FinishUnsuccessfully)))
    (elif (and (> (.roll (Variables|/Script/Engine.SceneComponent|GetRelativeRotation (Variables|Default|Getfbx_Moon))) (- _correctposition 15.0)) (< (.roll (Variables|/Script/Engine.SceneComponent|GetRelativeRotation (Variables|Default|Getfbx_Moon))) (+ _correctposition 15.0)))
      (goto _label)
      (else
        (Default|LogExperimentSolutionAttempt (Variables|Default|GetLogger) (Variables|/Game/Blueprints/BP_ExperimentDesk.BP_ExperimentDesk_C|GetSessionID _table) "NewEnumerator0" (Variables|/Game/Blueprints/BP_ExperimentDesk.BP_ExperimentDesk_C|GetExperimentID _table) (Variables|/Game/Blueprints/BP_ExperimentDesk.BP_ExperimentDesk_C|GetChosenDifficulty _table) "NewEnumerator1")
        (CallFunction|FinishUnsuccessfully)))))

(event Custom|SetAutoCheck
  (params (isChecked :type Boolean))
  (Variables|Default|SetisAutoCheckOn isChecked))

(event Custom|OnCheckButtonPressed
  (if (Variables|Default|GetisExperimentActive)
    (CallFunction|CheckforCorrectMoonPosition)
    (Variables|Default|SetisMoonGrabbed false)))

(event Custom|SetMoonphasesView
  (params (MoonphaseView :type Moon%20Experiment%20View%20Object%20Reference))
  (Variables|Default|SetUIMoonPhaseInstruction MoonphaseView))

(event EventBeginPlay
  (Transformation|SetRelativeRotation (Variables|Default|Getfbx_Moon) (Math|Rotator|MakeRotator (Math|Random|RandomFloatinRange -1.7e+02 1.7e+02) 0.0 0.0) false false))

(event EventMouseTouch
  (Variables|Default|SetisGrabbedByMouse true))

(event EventTick
  (params (DeltaSeconds :type Float%20%28single-precision%29))
  (bind _returnvalue (Game|GetPlayerController 0))
  (bind (_locationx _locationy) (Game|Player|GetMousePosition _returnvalue))
  (if (Variables|Default|GetisExperimentActive)
    (if (Variables|Default|GetisGrabbedByMouse)
      (bind (_returnvalue_2 _returnvalue2 _returnvalue3) (CallFunction|CalculateMoonRotationAccordingtoFingerLocation (Math|Vector|MakeVector _locationx _locationy 0.0)))
      (if _returnvalue2
        (Transformation|SetRelativeRotation (Variables|Default|Getfbx_Moon) (Math|Rotator|MakeRotator _returnvalue_2 0.0 0.0) false false)
        (else
          (Transformation|SetRelativeRotation (Variables|Default|Getfbx_Moon) (Math|Rotator|MakeRotator _returnvalue3 0.0 0.0) false false))))
    (else
      (Transformation|SetRelativeRotation (Variables|Default|Getfbx_Moon) (Math|Rotator|MakeRotator (+ (.roll (Variables|/Script/Engine.SceneComponent|GetRelativeRotation (Variables|Default|Getfbx_Moon))) 0.05) 0.0 0.0) false false))))

(event EventTouchInteract
  (params (Location :type Vector :default "0, 0, 0"))
  (if (Variables|Default|GetisExperimentActive)
    (Variables|Default|SetisMoonGrabbed true)
    (bind (_returnvalue _returnvalue2 _returnvalue3) (CallFunction|CalculateMoonRotationAccordingtoFingerLocation Location))
    (if _returnvalue2
      (Transformation|SetRelativeRotation (Variables|Default|Getfbx_Moon) (Math|Rotator|MakeRotator _returnvalue 0.0 0.0) false false)
      (else
        (Transformation|SetRelativeRotation (Variables|Default|Getfbx_Moon) (Math|Rotator|MakeRotator _returnvalue3 0.0 0.0) false false)))))

(event EventOnActivateExperiment
  (|CallParentFunction)
  (Utilities|Array|Clear (Variables|Default|GetMoonPhasesForCurrentDifficulty))
  (if (Utilities|IsValid (Variables|Default|GetUIMoonPhaseInstruction))
    (EventDispatchers|BindEventtoCheckButtonPressed (Variables|Default|GetUIMoonPhaseInstruction) (delegate Custom|OnCheckButtonPressed))
    (UserInterface|Viewport|AddtoViewport (Variables|Default|GetUIMoonPhaseInstruction) 0))
  (switch Utilities|FlowControl|Switch|SwitchonExperimentDifficulty (Variables|Default|GetDifficulty)
    (:NewEnumerator0
      (for _array_element (Variables|Default|GetMoonPhases)
        (if (Utilities|Enum|Equal(Enum) (.Difficulty (Utilities|Struct|BreakMoonPhase _array_element)) "NewEnumerator0")
          (Utilities|Array|Add (Variables|Default|GetMoonPhasesForCurrentDifficulty) _array_element)))
      (Utilities|Array|Shuffle (Variables|Default|GetMoonPhasesForCurrentDifficulty))
      (CallFunction|SetNewMoonPhase))
    (:NewEnumerator1
      (for _array_element_2 (Variables|Default|GetMoonPhases)
        (if (or (Utilities|Enum|Equal(Enum) (.Difficulty (Utilities|Struct|BreakMoonPhase _array_element_2)) "NewEnumerator0") (Utilities|Enum|Equal(Enum) (.Difficulty (Utilities|Struct|BreakMoonPhase _array_element_2)) "NewEnumerator1"))
          (Utilities|Array|Add (Variables|Default|GetMoonPhasesForCurrentDifficulty) _array_element_2)))
      (Utilities|Array|Shuffle (Variables|Default|GetMoonPhasesForCurrentDifficulty))
      (CallFunction|SetNewMoonPhase))
    (:NewEnumerator2
      (bind _output_get (Variables|Default|SetMoonPhasesForCurrentDifficulty (Variables|Default|GetMoonPhases)))
      (Utilities|Array|Shuffle _output_get)
      (CallFunction|SetNewMoonPhase))))

(event EventOnDeactivateExperiment
  (|CallParentFunction)
  (Variables|Default|SetCurrentMoonPhaseIndex 0)
  (Variables|Default|SetCurrentMoonPhase "")
  (Utilities|Array|Clear (Variables|Default|GetMoonPhasesForCurrentDifficulty))
  (Default|DisableMenu (Variables|Default|GetUIMoonPhaseInstruction)))

(event EventTouchMoveInteract
  (params (Location :type Vector :default "0, 0, 0"))
  (if (Variables|Default|GetisExperimentActive)
    (Variables|Default|SetisMoonGrabbed true)
    (bind (_returnvalue _returnvalue2 _returnvalue3) (CallFunction|CalculateMoonRotationAccordingtoFingerLocation Location))
    (if _returnvalue2
      (Transformation|SetRelativeRotation (Variables|Default|Getfbx_Moon) (Math|Rotator|MakeRotator _returnvalue 0.0 0.0) false false)
      (else
        (Transformation|SetRelativeRotation (Variables|Default|Getfbx_Moon) (Math|Rotator|MakeRotator _returnvalue3 0.0 0.0) false false)))))

(event EventTouchRelease
  (if (Variables|Default|GetisExperimentActive)
    (if (Variables|Default|GetisAutoCheckOn)
      (CallFunction|CheckforCorrectMoonPosition)
      (Variables|Default|SetisMoonGrabbed false))))

(event EventMouseTouchRelease
  (Variables|Default|SetisGrabbedByMouse false)
  (if (Variables|Default|GetisExperimentActive)
    (if (Variables|Default|GetisAutoCheckOn)
      (CallFunction|CheckforCorrectMoonPosition))))

(fn ConstructionScript)

(fn CalculateMoonRotationAccordingtoFingerLocation
  (params (A :type Vector))
  (bind _returnvalue (Game|GetPlayerController 0))
  (bind _returnvalue_2 (Class|KismetMathLibrary|VectorNormal2D "-1.000000,0.000000,1.000000" 0.0001))
  (bind _fbx_earth (Variables|Default|Getfbx_Earth))
  (bind _returnvalue_3 (Transformation|GetWorldLocation _fbx_earth))
  (bind _screenposition (Class|GameplayStatics|ProjectWorldtoScreen _returnvalue _returnvalue_3 false))
  (bind _returnvalue_4 (- A _screenposition))
  (bind _returnvalue_5 (Class|KismetMathLibrary|VectorNormal2D _returnvalue_4 0.0001))
  (bind _returnvalue_6 (Math|Vector|DotProduct _returnvalue_2 _returnvalue_5))
  (bind _returnvalue_7 (Class|KismetMathLibrary|DegAcos _returnvalue_6))
  (return (+ (- 1.8e+02 _returnvalue_7) 1.8e+02) (> (Math|Trig|Sin(Degrees) (Math|Vector|DotProduct (Class|KismetMathLibrary|VectorNormal2D "0.000000,-1.000000,1.000000" 0.0001) _returnvalue_5)) 0.0) _returnvalue_7))