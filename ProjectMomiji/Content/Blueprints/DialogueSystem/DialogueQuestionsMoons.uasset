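; Dialogue Blueprint for the NPC Mori in the moon experiment, with German lines.
; The Dialogue override calls its parent, then shows one line congratulating the player and suggesting a shop color purchase, before clearing progress and closing the conversation.
; An unconnected, never-executed branch holds a two-question moon quiz per difficulty, with corrective feedback and a shared closing line.
; The Hard questions in that branch are placeholder text.
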(fn Dialogue
  (params (ExperimentDifficulty :type ExperimentDifficulty%20Enum :default "NewEnumerator0"))
  (|CallParentFunction ExperimentDifficulty)
  (bind _state (CallFunction|AddDialogue "Mori" "Hey, toll, dass du das Experiment schon gelöst hast! Wenn du möchtest, könntest du nun für mich eine neue Farbe im Shop kaufen!" (Utilities|Array|MakeArray "Danke für die Info!")))
  (switch Utilities|FlowControl|Switch|SwitchonDialogueState _state
    (:NewEnumerator0
      (CallFunction|ClearDialogueProgress)
      (CallFunction|CloseConversation))))