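; Dialogue Blueprint for a German post-experiment quiz in which the NPC Mori asks the player about sound frequency, amplitude and phase shift.
; ExperimentDifficulty selects the branch: Easy and Medium ask two multiple-choice questions, Hard asks three.
; Each answer's OptionIndex leads to a confirming or correcting line, and both continue onward without scoring.
; All branches converge on a farewell mentioning shop coins, then clear dialogue progress and close the conversation.
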(fn Dialogue
  (params (ExperimentDifficulty :type ExperimentDifficulty%20Enum :default "NewEnumerator0"))
  (|CallParentFunction ExperimentDifficulty)
  (bind _state (CallFunction|AddDialogue "Mori" "Hey, toll, dass du das Frequenzen Experiment schon geschafft hast! Ich habe es selbst nicht ganz verstanden. Kann ich dir ein paar Fragen stellen? Vielleicht kannst du sie mir ja erklären." (Utilities|Array|MakeArray "Okay")))
  (switch Utilities|FlowControl|Switch|SwitchonDialogueState _state
    (:NewEnumerator0
      (switch Utilities|FlowControl|Switch|SwitchonExperimentDifficulty ExperimentDifficulty
        (:NewEnumerator0
          (bind (_state_2 _optionindex) (CallFunction|AddDialogue "Mori" "Meine erste Frage wäre:  Wie verändert sich eine Frequenzkurve, wenn man die Frequenz verändert?" (Utilities|Array|MakeArray "Die Höhe der Kurve wird höher oder niedriger" "Die Intervalle der Kurve werden länger oder kürzer" "Die Kurve verschiebt sich von links nach rechts")))
          (switch Utilities|FlowControl|Switch|SwitchonDialogueState _state_2
            (:NewEnumerator0
              (switch int _optionindex
                (:0
                  (bind _state_3 (CallFunction|AddDialogue "Mori" "Ich denke leider nicht, dass das stimmt. Wenn ich mich richtig erinnere werden die Intervalle länger oder kürzer." (Utilities|Array|MakeArray "Okay, schau ich mir nocheinmal an!") :!label _label))
                  (switch Utilities|FlowControl|Switch|SwitchonDialogueState _state_3
                    (:NewEnumerator0
                      _)))
                (:1
                  (bind _state_4 (CallFunction|AddDialogue "Mori" "Genau stimmt! Jetzt kann ich mich wieder erinnern! Natürlich werden die Intervalle länger oder kürzer." (Utilities|Array|MakeArray "Toll, nächste Frage!")))
                  (switch Utilities|FlowControl|Switch|SwitchonDialogueState _state_4
                    (:NewEnumerator0
                      _)))
                (:2
                  (goto _label)))
              (bind (_state_5 _optionindex_2) (CallFunction|AddDialogue "Mori" "Zweite Frage:  Wie verändert sich eine Ton, wenn man die Frequenz verändert?" (Utilities|Array|MakeArray "Er verändert sich granicht" "Er wird Lauter oder Leiser" "Er wird höher oder tiefer")))
              (switch Utilities|FlowControl|Switch|SwitchonDialogueState _state_5
                (:NewEnumerator0
                  (switch int _optionindex_2
                    (:0
                      (bind _state_6 (CallFunction|AddDialogue "Mori" "Ich denke leider nicht, dass das stimmt. Wenn ich mich richtig erinnere wird der Ton höher oder tiefer." (Utilities|Array|MakeArray "Okay, schau ich mir nocheinmal an!") :!label _label_2))
                      (switch Utilities|FlowControl|Switch|SwitchonDialogueState _state_6
                        (:NewEnumerator0
                          _)))
                    (:1
                      (goto _label_2))
                    (:2
                      (bind _state_7 (CallFunction|AddDialogue "Mori" "Genau stimmt! Jetzt kann ich mich wieder erinnern! Natürlich wird der Ton höher oder tiefer!" (Utilities|Array|MakeArray "Toll, nächste Frage!")))
                      (switch Utilities|FlowControl|Switch|SwitchonDialogueState _state_7
                        (:NewEnumerator0
                          _)))))))))
        (:NewEnumerator1
          (bind (_state_8 _optionindex_3) (CallFunction|AddDialogue "Mori" "Meine erste Frage wäre: Wenn ich die Lautstärke eines Tons verändern will, welchen wert muss ich dann anpassen?" (Utilities|Array|MakeArray "Den Wert der Phasenverschiebung" "Den Wert der Frequenz" "Den Wert der Amplitude")))
          (switch Utilities|FlowControl|Switch|SwitchonDialogueState _state_8
            (:NewEnumerator0
              (switch int _optionindex_3
                (:0
                  (bind _state_9 (CallFunction|AddDialogue "Mori" "Ich denke leider nicht, dass das stimmt. Wenn ich mich richtig erinnere ist doch die Amplitude für die Lautstärke verantwortlich." (Utilities|Array|MakeArray "Okay, schau ich mir nocheinmal an!") :!label _label_3))
                  (switch Utilities|FlowControl|Switch|SwitchonDialogueState _state_9
                    (:NewEnumerator0
                      _)))
                (:1
                  (goto _label_3))
                (:2
                  (bind _state_10 (CallFunction|AddDialogue "Mori" "Genau stimmt! Jetzt kann ich mich wieder erinnern! Natürlich muss ich die Amplitude anpassen, wenn ich die Lautstärke verändern will." (Utilities|Array|MakeArray "Toll, nächste Frage!")))
                  (switch Utilities|FlowControl|Switch|SwitchonDialogueState _state_10
                    (:NewEnumerator0
                      _))))
              (bind (_state_11 _optionindex_4) (CallFunction|AddDialogue "Mori" "Zweite Frage: Wenn ich die Amplitude verändere, wie verändert sich dann die Frequenzkurve?" (Utilities|Array|MakeArray "Die Höhe der Kurve wird höher oder niedriger" "Die Intervalle der Kurve werden länger oder kürzer" "Die Kurve verschiebt sich von links nach rechts")))
              (switch Utilities|FlowControl|Switch|SwitchonDialogueState _state_11
                (:NewEnumerator0
                  (switch int _optionindex_4
                    (:0
                      (bind _state_12 (CallFunction|AddDialogue "Mori" "Genau stimmt! Jetzt kann ich mich wieder erinnern! Natürlich ändert die Amplitude die Höhe der Kurve!" (Utilities|Array|MakeArray "Toll, nächste Frage!")))
                      (switch Utilities|FlowControl|Switch|SwitchonDialogueState _state_12
                        (:NewEnumerator0
                          _)))
                    (:1
                      (bind _state_13 (CallFunction|AddDialogue "Mori" "Ich denke leider nicht, dass das stimmt. Wenn ich mich richtig erinnere ändert die Amplitude die Höhe der Kurve." (Utilities|Array|MakeArray "Okay, schau ich mir nocheinmal an!") :!label _label_4))
                      (switch Utilities|FlowControl|Switch|SwitchonDialogueState _state_13
                        (:NewEnumerator0
                          _)))
                    (:2
                      (goto _label_4))))))))
        (:NewEnumerator2
          (bind (_state_14 _optionindex_5) (CallFunction|AddDialogue "Mori" "Meine erste Frage wäre: Wenn ich einen sehr hohen Ton höre, und ihn tiefer Stellen möchte, was muss ich tun?" (Utilities|Array|MakeArray "Den Wert der Phasenversschiebung erhöhen" "Den Wert der Phasenversschiebung verringern" "Den Wert der Frequenz erhöhen" "Den Wert der Frequenz verringern" "Den Wert der Amplitude erhöhen" "Den Wert der Amplitude verringern")))
          (switch Utilities|FlowControl|Switch|SwitchonDialogueState _state_14
            (:NewEnumerator0
              (switch int _optionindex_5
                (:0
                  (bind _state_15 (CallFunction|AddDialogue "Mori" "Ich denke leider nicht, dass das stimmt. Wenn ich mich richtig erinnere müsste ich doch die Frequenz verringern, um den Ton niedriger zu machen." (Utilities|Array|MakeArray "Okay, schau ich mir nocheinmal an!") :!label _label_5))
                  (switch Utilities|FlowControl|Switch|SwitchonDialogueState _state_15
                    (:NewEnumerator0
                      _)))
                (:1
                  (goto _label_5))
                (:2
                  (goto _label_5))
                (:3
                  (bind _state_16 (CallFunction|AddDialogue "Mori" "Genau stimmt! Jetzt kann ich mich wieder erinnern! Natürlich müsste ich die Frequenz veringern um einen Ton tiefer zu machen." (Utilities|Array|MakeArray "Toll!")))
                  (switch Utilities|FlowControl|Switch|SwitchonDialogueState _state_16
                    (:NewEnumerator0
                      _)))
                (:4
                  (goto _label_5))
                (:5
                  (goto _label_5)))
              (bind (_state_17 _optionindex_6) (CallFunction|AddDialogue "Mori" "Meine zweite Frage wäre: Wenn ich sehr Laute Musik höre, und ich sie Leiser drehen möchte, welchen Wert muss ich dann anpassen?" (Utilities|Array|MakeArray "Den Wert der Phasenversschiebung erhöhen" "Den Wert der Phasenversschiebung verringern" "Den Wert der Frequenz erhöhen" "Den Wert der Frequenz verringern" "Den Wert der Amplitude erhöhen" "Den Wert der Amplitude verringern")))
              (switch Utilities|FlowControl|Switch|SwitchonDialogueState _state_17
                (:NewEnumerator0
                  (switch int _optionindex_6
                    (:0
                      (bind _state_18 (CallFunction|AddDialogue "Mori" "Ich denke leider nicht, dass das stimmt. Wenn ich mich richtig erinnere müsste ich doch den Wert der Amplitude erinnern." (Utilities|Array|MakeArray "Okay, schau ich mir nocheinmal an!") :!label _label_6))
                      (switch Utilities|FlowControl|Switch|SwitchonDialogueState _state_18
                        (:NewEnumerator0
                          _)))
                    (:1
                      (goto _label_6))
                    (:2
                      (goto _label_6))
                    (:3
                      (goto _label_6))
                    (:4
                      (goto _label_6))
                    (:5
                      (bind _state_19 (CallFunction|AddDialogue "Mori" "Genau stimmt! Jetzt kann ich mich wieder erinnern! Natürlich müsste den Wert der Amplituder verringern!" (Utilities|Array|MakeArray "Toll!")))
                      (switch Utilities|FlowControl|Switch|SwitchonDialogueState _state_19
                        (:NewEnumerator0
                          _))))
                  (bind (_state_20 _optionindex_7) (CallFunction|AddDialogue "Mori" "Dritte Frage: Wie verändert die Phasenverschiebung, die Frequenzkurve?" (Utilities|Array|MakeArray "Die Höhe der Kurve wird höher oder niedriger" "Die Intervalle der Kurve werden länger oder kürzer" "Die Kurve entspringt an einem anderen Wert entlang der Y-Achse")))
                  (switch Utilities|FlowControl|Switch|SwitchonDialogueState _state_20
                    (:NewEnumerator0
                      (switch int _optionindex_7
                        (:0
                          (bind _state_21 (CallFunction|AddDialogue "Mori" "Ich denke leider nicht, dass das stimmt. Wenn ich mich richtig erinnere lässt die Phasenverschiebung die Kurve an einem anderen Punkt an der Y-Achse entspringen." (Utilities|Array|MakeArray "Okay, schau ich mir nocheinmal an!") :!label _label_7))
                          (switch Utilities|FlowControl|Switch|SwitchonDialogueState _state_21
                            (:NewEnumerator0
                              _)))
                        (:1
                          (goto _label_7))
                        (:2
                          (bind _state_22 (CallFunction|AddDialogue "Mori" "Genau stimmt! Jetzt kann ich mich wieder erinnern! Natürlich lässt die Phasenverschiebung die Kurve an einem anderen Punkt an der Y-Achse entspringen." (Utilities|Array|MakeArray "Toll, nächste Frage!")))
                          (switch Utilities|FlowControl|Switch|SwitchonDialogueState _state_22
                            (:NewEnumerator0
                              _))))))))))))
      (bind _state_23 (CallFunction|AddDialogue "Mori" "Das wars! Danke dass du meine Fragen beantwortet hast! Und vergiss nicht, deine tollen Münzen im Shop auszugeben!" (Utilities|Array|MakeArray "Gerne!")))
      (switch Utilities|FlowControl|Switch|SwitchonDialogueState _state_23
        (:NewEnumerator0
          (CallFunction|ClearDialogueProgress)
          (CallFunction|CloseConversation))))))