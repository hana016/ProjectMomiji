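; DialogueIntroduction is the intro conversation in which the companion Mori greets the player in German and explains the game.
; Mori covers the three experiment tables, the coins that buy cosmetics for Mori, and tapping Mori for help.
; After calling the parent Dialogue, it chains five single-option AddDialogue steps through their Pass Through states.
; The final step clears dialogue progress and closes the conversation.
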(fn Dialogue
  (params (ExperimentDifficulty :type ExperimentDifficulty%20Enum :default "NewEnumerator0"))
  (|CallParentFunction "NewEnumerator0")
  (bind _state (CallFunction|AddDialogue "Mori" "Hey, ich bin Mori! Ich bin dein Begleiter heute in diesem Spiel! Es freut mich dich kennenzulernen!" (Utilities|Array|MakeArray "Hallo Mori! Freut mich auch dich kennenzulernen!")))
  (switch Utilities|FlowControl|Switch|SwitchonDialogueState _state
    (:NewEnumerator0
      (bind _state_2 (CallFunction|AddDialogue "Mori" "Deine Aufgabe heute ist es alle 3 Experimenttische zu besuchen und mindestens ein Experiment an jedem Tisch erfolgreich zu lösen. Die Tische die ich meine sind direkt hinter mir zu finden. Du kannst sie erkennen an den grünen Hologrammen oben drauf." (Utilities|Array|MakeArray "Okay!")))
      (switch Utilities|FlowControl|Switch|SwitchonDialogueState _state_2
        (:NewEnumerator0
          (bind _state_3 (CallFunction|AddDialogue "Mori" "Nach jedem Experiment, dass du erfolgreich abgeschlossen hast, bekommst du eine Münze. Mit diesen Münzen kannst du Farben und Muster für mein Aussehen kaufen. Ich würde mich sehr über einen neuen Anstrich freuen!" (Utilities|Array|MakeArray "Verstanden!")))
          (switch Utilities|FlowControl|Switch|SwitchonDialogueState _state_3
            (:NewEnumerator0
              (bind _state_4 (CallFunction|AddDialogue "Mori" "Fals du Fragen hast, kannst du immer zu mir kommen, mich antippen und ich versuche dir das Experiment genauer zu erklären." (Utilities|Array|MakeArray "Werde ich machen.")))
              (switch Utilities|FlowControl|Switch|SwitchonDialogueState _state_4
                (:NewEnumerator0
                  (bind _state_5 (CallFunction|AddDialogue "Mori" "Na dann viel Spaß! Und ich werde immer bei dir bleiben, fals du Hilfe benötigst!" (Utilities|Array|MakeArray "Danke!")))
                  (switch Utilities|FlowControl|Switch|SwitchonDialogueState _state_5
                    (:NewEnumerator0
                      (CallFunction|ClearDialogueProgress)
                      (CallFunction|CloseConversation))))))))))))