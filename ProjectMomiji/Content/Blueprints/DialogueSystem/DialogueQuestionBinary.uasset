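; Mori NPC dialogue for the binary-number experiment, overriding Dialogue to congratulate the player on solving it and suggest other difficulties or experiments.
; After the parent call, one AddDialogue line plays, then progress clears and the conversation closes.
; A disconnected, never-run branch holds a German two-question quiz per difficulty, with right/wrong feedback converging on a shared farewell.
; In that branch, some Easy answers are unwired and Hard feedback repeats Medium's answers.
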(fn Dialogue
  (params (ExperimentDifficulty :type ExperimentDifficulty%20Enum :default "NewEnumerator0"))
  (|CallParentFunction ExperimentDifficulty)
  (bind _state (CallFunction|AddDialogue "Mori" "Hey, toll, dass du das Experiment schon gelöst hast! Wenn du möchtest, könntest du nun die anderen Schwierigkeiten oder Experimente ausprobieren!" (Utilities|Array|MakeArray "Okay")))
  (switch Utilities|FlowControl|Switch|SwitchonDialogueState _state
    (:NewEnumerator0
      (CallFunction|ClearDialogueProgress)
      (CallFunction|CloseConversation))))