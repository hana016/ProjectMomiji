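; BP_ExperimentDesk is an interactive table where the player picks a difficulty and plays one of three experiments of a moon phase, binary or frequency type.
; It creates all menu widgets on BeginPlay and swaps them through difficulty, description and reward or fail screens, driven by bound events.
; Starting moves the player camera to the chosen experiment, and success awards a saved coin.
; Table sessions and experiment attempts are logged with IDs.
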(event OnComponentBeginOverlap(InteractionArea)
  (params (OverlappedComponent :type Primitive%20Component%20Object%20Reference) (OtherActor :type Actor%20Object%20Reference) (OtherComp :type Primitive%20Component%20Object%20Reference) (OtherBodyIndex :type Integer) (bFromSweep :type Boolean) (SweepResult :type Hit%20Result%20Structure%20%28by%20ref%29))
  (if (Actor|ActorHasTag OtherActor "Player")
    (CallFunction|EnableMenuView "NewEnumerator4" true)
    (Default|CallPlayerIsNear (Variables|Default|GetExperimentType))))

(event OnComponentEndOverlap(InteractionArea)
  (params (OverlappedComponent :type Primitive%20Component%20Object%20Reference) (OtherActor :type Actor%20Object%20Reference) (OtherComp :type Primitive%20Component%20Object%20Reference) (OtherBodyIndex :type Integer))
  (if (Actor|ActorHasTag OtherActor "Player")
    (CallFunction|EnableMenuView "NewEnumerator4" false)
    (Default|CallPlayerLeft)))

(event Custom|ActivateEasyDifficulty
  (Variables|Default|SetChosenDifficulty "NewEnumerator0")
  (CallFunction|SetupExperimentDescriptionInformation)
  (CallFunction|DisableAllMenus)
  (CallFunction|EnableMenuView "NewEnumerator1" true))

(event Custom|ActivateMediumDifficulty
  (Variables|Default|SetChosenDifficulty "NewEnumerator1")
  (CallFunction|SetupExperimentDescriptionInformation)
  (CallFunction|DisableAllMenus)
  (CallFunction|EnableMenuView "NewEnumerator1" true))

(event Custom|SetMusic
  (params (MusicOn :type Boolean))
  (for _array_element (Variables|Default|GetExperiments)
    (bind _asbp_frequency_experiment (Utilities|Casting|CastToBP_FrequencyExperiment _array_element))
    (Default|SetMusic _asbp_frequency_experiment MusicOn)))

(event Custom|ActivateHardDifficulty
  (Variables|Default|SetChosenDifficulty "NewEnumerator2")
  (CallFunction|SetupExperimentDescriptionInformation)
  (CallFunction|DisableAllMenus)
  (CallFunction|EnableMenuView "NewEnumerator1" true))

(event Custom|StartExperiment
  (CallFunction|ActivaateExperiment (Variables|Default|GetChosenDifficulty))
  (CallFunction|DisableAllMenus)
  (Default|LogExperimentStartandEnd (Variables|Default|GetLogger) "ES" (Variables|Default|GetSessionID) (Variables|Default|GetExperimentType) (Variables|Default|GetExperimentID) (Variables|Default|GetChosenDifficulty) "NewEnumerator3")
  (Variables|Default|SetisExperimentEndLogged false))

(event Custom|ShowRewardMenu
  (CallFunction|SetMostDifficultExperimentFinished)
  (CallFunction|SetupRewardInformation)
  (CallFunction|DisableAllMenus)
  (CallFunction|EnableMenuView "NewEnumerator2" true)
  (Variables|Default|SethasFinishedOneExperiment true)
  (Default|LogExperimentStartandEnd (Variables|Default|GetLogger) "EE" (Variables|Default|GetSessionID) (Variables|Default|GetExperimentType) (Variables|Default|GetExperimentID) (Variables|Default|GetChosenDifficulty) "NewEnumerator0")
  (Math|Integer|IncrementInt (Variables|Default|GetExperimentID)
    (:%20%20
      (Variables|Default|SetisExperimentEndLogged true))))

(event Custom|ShowFailMenu
  (CallFunction|DisableAllMenus)
  (CallFunction|EnableMenuView "NewEnumerator3" true)
  (Default|LogExperimentStartandEnd (Variables|Default|GetLogger) "EE" (Variables|Default|GetSessionID) (Variables|Default|GetExperimentType) (Variables|Default|GetExperimentID) (Variables|Default|GetChosenDifficulty) "NewEnumerator1")
  (Variables|Default|SetisExperimentEndLogged true)
  (Math|Integer|IncrementInt (Variables|Default|GetExperimentID)))

(event Custom|ShowDifficultyMenu
  (CallFunction|DisableAllMenus)
  (CallFunction|EnableMenuView "NewEnumerator0" true))

(event Custom|ShowHelpMenu
  (Default|ActivateHelpPage (Variables|Default|GetFailMenu) (Variables|Default|GetExperimentType))
  (Audio|PlaySound2D "/Game/Sounds/DuSchaffstDas_.DuSchaffstDas_" 1.0 1.0 0.0 0 0))

(event Custom|SetAutoCheck
  (params (isChecked :type Boolean))
  (for _array_element (Variables|Default|GetExperiments)
    (bind _asbp_moon_experiemnt (Utilities|Casting|CastToBP_MoonExperiemnt _array_element))
    (Default|SetAutoCheck _asbp_moon_experiemnt isChecked)))

(event EventBeginPlay
  ;[1 1 1] Initialize All Menus
  (CallFunction|InitMenuView "NewEnumerator0")
  (CallFunction|InitMenuView "NewEnumerator1")
  (CallFunction|InitMenuView "NewEnumerator2")
  (CallFunction|InitMenuView "NewEnumerator3")
  (CallFunction|InitMenuView "NewEnumerator4")
  (CallFunction|InitMenuView "NewEnumerator5")
  (CallFunction|InitMenuView "NewEnumerator6")
  (CallFunction|InitMenuView "NewEnumerator7")
  (EventDispatchers|BindEventtoCheckBoxClicked (Variables|Default|GetMoonphasesView) (delegate Custom|SetAutoCheck))
  (EventDispatchers|BindEventtoOnToggleMusic (Variables|Default|GetFrequencyView) (delegate Custom|SetMusic))
  (CallFunction|SetViewonExperiments)
  ;[1 1 1] Bind Events for Difficulty Menu
  (EventDispatchers|BindEventtoActivateEasyDifficulty (Variables|Default|GetDifficultyMenu) (delegate Custom|ActivateEasyDifficulty))
  (EventDispatchers|BindEventtoActivateMediumDifficulty (Variables|Default|GetDifficultyMenu) (delegate Custom|ActivateMediumDifficulty))
  (EventDispatchers|BindEventtoActivateHardDifficulty (Variables|Default|GetDifficultyMenu) (delegate Custom|ActivateHardDifficulty))
  (EventDispatchers|BindEventtoStartExperiment (Variables|Default|GetExperimentDescriptionMenu) (delegate Custom|StartExperiment))
  ;[1 1 1] Bind Events for Reward Menu
  (EventDispatchers|BindEventtoStartExperiment (Variables|Default|GetRewardMenu) (delegate Custom|StartExperiment))
  (EventDispatchers|BindEventtoEndExperiment (Variables|Default|GetRewardMenu) (delegate EventCancelInteracation))
  (EventDispatchers|BindEventtoGotoDifficultyMenu (Variables|Default|GetRewardMenu) (delegate Custom|ShowDifficultyMenu))
  ;[1 1 1] Bind Events for FailMenu
  (EventDispatchers|BindEventtoStartExperiment (Variables|Default|GetFailMenu) (delegate Custom|StartExperiment))
  (EventDispatchers|BindEventtoEndExperiment (Variables|Default|GetFailMenu) (delegate EventCancelInteracation))
  (EventDispatchers|BindEventtoGotoDifficultyMenu (Variables|Default|GetFailMenu) (delegate Custom|ShowDifficultyMenu))
  (EventDispatchers|BindEventtoShowHelpPage (Variables|Default|GetFailMenu) (delegate Custom|ShowHelpMenu))
  ;[1 1 1] Bind Events for all Experiments
  (for _array_element (Variables|Default|GetExperiments)
    (EventDispatchers|BindEventtoFinishedSuccessfully _array_element (delegate Custom|ShowRewardMenu))
    (EventDispatchers|BindEventtoFinishedUnsuccessfully _array_element (delegate Custom|ShowFailMenu))))

(event EventActivate
  (Variables|Default|SetisActive true))

(event EventDeactivate
  (Variables|Default|SetisActive false))

(event EventButtonInteract
  (if (Variables|Default|GetisActive)
    (CallFunction|DisableAllMenus)
    (if (Utilities|IsValid (Variables|Default|GetPlayerCharacter))
      _
      (else
        (bind _asbp_first_person_character (Utilities|Casting|CastToBP_FirstPersonCharacter (Game|GetPlayerCharacter 0)))
        (Variables|Default|SetPlayerCharacter _asbp_first_person_character)))
    (if (not (Variables|Default|GetisTableActive))
      (Default|SwitchMobileControlls (Variables|Default|GetPlayerCharacter) "NewEnumerator3")
      (CallFunction|EnableMenuView "NewEnumerator0" true)
      (Default|LogTableStartandEnd (Variables|Default|GetLogger) "TS" (Variables|Default|GetSessionID) (Variables|Default|GetExperimentType)))))

(event EventCancelInteracation
  (Variables|Default|SetisTableActive false)
  (Default|MoveCamera (Variables|Default|GetPlayerCharacter) 0 true)
  (CallFunction|DisableAllMenus)
  (Default|EnableCoinView (Variables|Default|GetPlayerCharacter) true)
  (for _array_element (Variables|Default|GetExperiments)
    (Default|DeactivateExperiment _array_element))
  (if (Variables|Default|GethasFinishedOneExperiment)
    (Variables|Default|SethasFinishedOneExperiment false)
    (Default|CallLeaveExperimentTable (Variables|Default|GetExperimentType))
    (Default|SwitchMobileControlls (Variables|Default|GetPlayerCharacter) "NewEnumerator2")
    (if (Variables|Default|GetisExperimentEndLogged)
      _
      (else
        (Default|LogExperimentStartandEnd (Variables|Default|GetLogger) "EE" (Variables|Default|GetSessionID) (Variables|Default|GetExperimentType) (Variables|Default|GetExperimentID) (Variables|Default|GetChosenDifficulty) "NewEnumerator2")
        (Variables|Default|SetisExperimentEndLogged true)
        (Math|Integer|IncrementInt (Variables|Default|GetExperimentID)
          (:%20%20
            _))))
    (Default|LogTableStartandEnd (Variables|Default|GetLogger) "TE" (Variables|Default|GetSessionID) (Variables|Default|GetExperimentType))
    (Math|Integer|IncrementInt (Variables|Default|GetSessionID))
    (else
      (Default|SwitchMobileControlls (Variables|Default|GetPlayerCharacter) "NewEnumerator0"))))

(fn ConstructionScript)

(fn ActivaateExperiment
  (params (Difficulty :type ExperimentDifficulty%20Enum :default "NewEnumerator0"))
  (bind _experiments (Variables|Default|GetExperiments))
  (bind _experiments_2 (Variables|Default|GetExperiments))
  (bind _experiments_3 (Variables|Default|GetExperiments))
  (bind _output (Utilities|Array|Get(acopy) _experiments_2))
  (bind _output_2 (Utilities|Array|Get(acopy) _experiments_3 1))
  (bind _output_3 (Utilities|Array|Get(acopy) _experiments 2))
  (switch Utilities|FlowControl|Switch|SwitchonExperimentDifficulty Difficulty
    (:NewEnumerator0
      (Default|MoveCamera (Variables|Default|GetPlayerCharacter) _output false)
      (Default|ActivateExperiment _output))
    (:NewEnumerator1
      (Default|MoveCamera (Variables|Default|GetPlayerCharacter) _output_2 false)
      (Default|ActivateExperiment _output_2))
    (:NewEnumerator2
      (Default|MoveCamera (Variables|Default|GetPlayerCharacter) _output_3 false)
      (Default|ActivateExperiment _output_3)))
  (Default|CallActivateExperiment))

(fn EnableMenuView
  (params (MenuType :type MenuType%20Enum :default "NewEnumerator0") (setEnabled :type Boolean))
  (bind _playercharacter (Variables|Default|GetPlayerCharacter))
  (switch Utilities|FlowControl|Switch|SwitchonMenuType MenuType
    (:NewEnumerator0
      (if (Utilities|IsValid (Variables|Default|GetDifficultyMenu))
        _
        (else
          (bind _returnvalue (UserInterface|CreateWidget "/Game/Blueprints/Menus/DifficultyMenu.DifficultyMenu_C"))
          (Variables|Default|SetDifficultyMenu _returnvalue)))
      (if setEnabled
        (UserInterface|Viewport|AddtoViewport (Variables|Default|GetDifficultyMenu) 0)
        (else
          (Widget|RemovefromParent (Variables|Default|GetDifficultyMenu)))))
    (:NewEnumerator1
      (if (Utilities|IsValid (Variables|Default|GetExperimentDescriptionMenu))
        _
        (else
          (bind _returnvalue_2 (UserInterface|CreateWidget "/Game/Blueprints/Menus/ExperimentDescriptionMenu.ExperimentDescriptionMenu_C"))
          (Variables|Default|SetExperimentDescriptionMenu _returnvalue_2)))
      (if setEnabled
        (UserInterface|Viewport|AddtoViewport (Variables|Default|GetExperimentDescriptionMenu) 0)
        (else
          (Widget|RemovefromParent (Variables|Default|GetExperimentDescriptionMenu)))))
    (:NewEnumerator2
      (if (Utilities|IsValid (Variables|Default|GetRewardMenu))
        _
        (else
          (bind _returnvalue_3 (UserInterface|CreateWidget "/Game/Blueprints/Menus/RewardsMenu.RewardsMenu_C"))
          (Variables|Default|SetRewardMenu _returnvalue_3)))
      (if setEnabled
        (UserInterface|Viewport|AddtoViewport (Variables|Default|GetRewardMenu) 0)
        (Default|AddCoin _playercharacter (Variables|Default|GetChosenDifficulty) (Variables|Default|GetExperimentType))
        (Default|SaveCoins _playercharacter)
        (else
          (Widget|RemovefromParent (Variables|Default|GetRewardMenu)))))
    (:NewEnumerator3
      (if (Utilities|IsValid (Variables|Default|GetFailMenu))
        _
        (else
          (bind _returnvalue_4 (UserInterface|CreateWidget "/Game/Blueprints/Menus/FailMenu.FailMenu_C"))
          (Variables|Default|SetFailMenu _returnvalue_4)))
      (if setEnabled
        (UserInterface|Viewport|AddtoViewport (Variables|Default|GetFailMenu) 0)
        (Default|DisableHelpPages (Variables|Default|GetFailMenu))
        (else
          (Widget|RemovefromParent (Variables|Default|GetFailMenu)))))
    (:NewEnumerator4
      (if (Utilities|IsValid (Variables|Default|GetInteractionBillboard))
        _
        (else
          (bind _returnvalue_5 (UserInterface|CreateWidget "/Game/Blueprints/InteractBillboard.InteractBillboard_C"))
          (Variables|Default|SetInteractionBillboard _returnvalue_5)))
      (if setEnabled
        (UserInterface|Viewport|AddtoViewport (Variables|Default|GetInteractionBillboard) 0)
        (else
          (Widget|RemovefromParent (Variables|Default|GetInteractionBillboard)))))
    (:NewEnumerator5
      (if (Utilities|IsValid (Variables|Default|GetMoonphasesView))
        _
        (else
          (bind _returnvalue_6 (UserInterface|CreateWidget "/Game/Blueprints/Experiment1/MoonExperimentView.MoonExperimentView_C"))
          (Variables|Default|SetMoonphasesView _returnvalue_6)))
      (if setEnabled
        (UserInterface|Viewport|AddtoViewport (Variables|Default|GetMoonphasesView) 0)
        (else
          (Widget|RemovefromParent (Variables|Default|GetMoonphasesView)))))
    (:NewEnumerator6
      (if (Utilities|IsValid (Variables|Default|GetBinaryView))
        _
        (else
          (bind _returnvalue_7 (UserInterface|CreateWidget "/Game/Blueprints/Experiment2/BinarExperimentView.BinarExperimentView_C"))
          (Variables|Default|SetBinaryView _returnvalue_7)))
      (if setEnabled
        (UserInterface|Viewport|AddtoViewport (Variables|Default|GetBinaryView) 0)
        (else
          (Widget|RemovefromParent (Variables|Default|GetBinaryView)))))
    (:NewEnumerator7
      (if (Utilities|IsValid (Variables|Default|GetFrequencyView))
        _
        (else
          (bind _returnvalue_8 (UserInterface|CreateWidget "/Game/Blueprints/Experiment3/FrequencyExperimentView.FrequencyExperimentView_C"))
          (Variables|Default|SetFrequencyView _returnvalue_8)))
      (if setEnabled
        (UserInterface|Viewport|AddtoViewport (Variables|Default|GetFrequencyView) 0)
        (else
          (Widget|RemovefromParent (Variables|Default|GetFrequencyView)))))))

(fn InitMenuView
  (params (MenuType :type MenuType%20Enum :default "NewEnumerator0"))
  (switch Utilities|FlowControl|Switch|SwitchonMenuType MenuType
    (:NewEnumerator0
      (if (not (Utilities|IsValid (Variables|Default|GetDifficultyMenu)))
        (bind _returnvalue (UserInterface|CreateWidget "/Game/Blueprints/Menus/DifficultyMenu.DifficultyMenu_C"))
        (bind _output_get (Variables|Default|SetDifficultyMenu _returnvalue))
        (Default|SetDifficultyImages _output_get (Utilities|Array|Get(acopy) (Variables|Default|GetDifficultyTextures)) (Utilities|Array|Get(acopy) (Variables|Default|GetDifficultyTextures) 1) (Utilities|Array|Get(acopy) (Variables|Default|GetDifficultyTextures) 2))))
    (:NewEnumerator1
      (if (not (Utilities|IsValid (Variables|Default|GetExperimentDescriptionMenu)))
        (bind _returnvalue_2 (UserInterface|CreateWidget "/Game/Blueprints/Menus/ExperimentDescriptionMenu.ExperimentDescriptionMenu_C"))
        (Variables|Default|SetExperimentDescriptionMenu _returnvalue_2)
        (Default|ChangeButtonColor _returnvalue_2 (Variables|Default|GetExperimentColor))))
    (:NewEnumerator2
      (if (not (Utilities|IsValid (Variables|Default|GetRewardMenu)))
        (bind _returnvalue_3 (UserInterface|CreateWidget "/Game/Blueprints/Menus/RewardsMenu.RewardsMenu_C"))
        (Variables|Default|SetRewardMenu _returnvalue_3)
        (Default|ChangeButtonColor _returnvalue_3 (Variables|Default|GetExperimentColor))))
    (:NewEnumerator3
      (if (not (Utilities|IsValid (Variables|Default|GetFailMenu)))
        (bind _returnvalue_4 (UserInterface|CreateWidget "/Game/Blueprints/Menus/FailMenu.FailMenu_C"))
        (Variables|Default|SetFailMenu _returnvalue_4)
        (Default|ChangeButtonColor _returnvalue_4 (Variables|Default|GetExperimentColor))))
    (:NewEnumerator4
      (if (not (Utilities|IsValid (Variables|Default|GetInteractionBillboard)))
        (bind _returnvalue_5 (UserInterface|CreateWidget "/Game/Blueprints/InteractBillboard.InteractBillboard_C"))
        (Variables|Default|SetInteractionBillboard _returnvalue_5)))
    (:NewEnumerator5
      (if (not (Utilities|IsValid (Variables|Default|GetMoonphasesView)))
        (bind _returnvalue_6 (UserInterface|CreateWidget "/Game/Blueprints/Experiment1/MoonExperimentView.MoonExperimentView_C"))
        (Variables|Default|SetMoonphasesView _returnvalue_6)))
    (:NewEnumerator6
      (if (not (Utilities|IsValid (Variables|Default|GetBinaryView)))
        (bind _returnvalue_7 (UserInterface|CreateWidget "/Game/Blueprints/Experiment2/BinarExperimentView.BinarExperimentView_C"))
        (Variables|Default|SetBinaryView _returnvalue_7)))
    (:NewEnumerator7
      (if (not (Utilities|IsValid (Variables|Default|GetFrequencyView)))
        (bind _returnvalue_8 (UserInterface|CreateWidget "/Game/Blueprints/Experiment3/FrequencyExperimentView.FrequencyExperimentView_C"))
        (Variables|Default|SetFrequencyView _returnvalue_8)))))

(fn SetupExperimentDescriptionInformation
  (bind _experiments (Variables|Default|GetExperiments))
  (bind _experiments_2 (Variables|Default|GetExperiments))
  (bind _experiments_3 (Variables|Default|GetExperiments))
  (bind _output (Utilities|Array|Get(acopy) _experiments_2 2))
  (bind _output_2 (Utilities|Array|Get(acopy) _experiments_3 1))
  (bind _output_3 (Utilities|Array|Get(acopy) _experiments))
  (switch Utilities|FlowControl|Switch|SwitchonExperimentDifficulty (Variables|Default|GetChosenDifficulty)
    (:NewEnumerator0
      (Default|SetupInformation (Variables|Default|GetExperimentDescriptionMenu) (Variables|/Game/Blueprints/BP_Experiment.BP_Experiment_C|GetExperimentName _output_3) (Variables|/Game/Blueprints/BP_Experiment.BP_Experiment_C|GetExperimentDescription _output_3) (Variables|/Game/Blueprints/BP_Experiment.BP_Experiment_C|GetNumberOfNeededCorrectAnswers _output_3) (Variables|/Game/Blueprints/BP_Experiment.BP_Experiment_C|GetExperimentTokenTexture _output_3)))
    (:NewEnumerator1
      (Default|SetupInformation (Variables|Default|GetExperimentDescriptionMenu) (Variables|/Game/Blueprints/BP_Experiment.BP_Experiment_C|GetExperimentName _output_2) (Variables|/Game/Blueprints/BP_Experiment.BP_Experiment_C|GetExperimentDescription _output_2) (Variables|/Game/Blueprints/BP_Experiment.BP_Experiment_C|GetNumberOfNeededCorrectAnswers _output_2) (Variables|/Game/Blueprints/BP_Experiment.BP_Experiment_C|GetExperimentTokenTexture _output_2)))
    (:NewEnumerator2
      (Default|SetupInformation (Variables|Default|GetExperimentDescriptionMenu) (Variables|/Game/Blueprints/BP_Experiment.BP_Experiment_C|GetExperimentName _output) (Variables|/Game/Blueprints/BP_Experiment.BP_Experiment_C|GetExperimentDescription _output) (Variables|/Game/Blueprints/BP_Experiment.BP_Experiment_C|GetNumberOfNeededCorrectAnswers _output) (Variables|/Game/Blueprints/BP_Experiment.BP_Experiment_C|GetExperimentTokenTexture _output)))))

(fn SetupRewardInformation
  (bind _experiments (Variables|Default|GetExperiments))
  (bind _experiments_2 (Variables|Default|GetExperiments))
  (bind _experiments_3 (Variables|Default|GetExperiments))
  (bind _output (Utilities|Array|Get(acopy) _experiments_2 2))
  (bind _output_2 (Utilities|Array|Get(acopy) _experiments_3))
  (bind _output_3 (Utilities|Array|Get(acopy) _experiments 1))
  (switch Utilities|FlowControl|Switch|SwitchonExperimentDifficulty (Variables|Default|GetChosenDifficulty)
    (:NewEnumerator0
      (Default|SetupMenuInformation (Variables|Default|GetRewardMenu) (Variables|/Game/Blueprints/BP_Experiment.BP_Experiment_C|GetExperimentTokenName _output_2) (Variables|/Game/Blueprints/BP_Experiment.BP_Experiment_C|GetExperimentTokenTexture _output_2)))
    (:NewEnumerator1
      (Default|SetupMenuInformation (Variables|Default|GetRewardMenu) (Variables|/Game/Blueprints/BP_Experiment.BP_Experiment_C|GetExperimentTokenName _output_3) (Variables|/Game/Blueprints/BP_Experiment.BP_Experiment_C|GetExperimentTokenTexture _output_3)))
    (:NewEnumerator2
      (Default|SetupMenuInformation (Variables|Default|GetRewardMenu) (Variables|/Game/Blueprints/BP_Experiment.BP_Experiment_C|GetExperimentTokenName _output) (Variables|/Game/Blueprints/BP_Experiment.BP_Experiment_C|GetExperimentTokenTexture _output)))))

(fn DisableAllMenus
  (Default|EnableCoinView (Variables|Default|GetPlayerCharacter) false)
  (CallFunction|EnableMenuView "NewEnumerator0" false)
  (CallFunction|EnableMenuView "NewEnumerator1" false)
  (CallFunction|EnableMenuView "NewEnumerator2" false)
  (CallFunction|EnableMenuView "NewEnumerator3" false)
  (CallFunction|EnableMenuView "NewEnumerator4" false))

(fn SetViewonExperiments
  (for _array_element (Variables|Default|GetExperiments)
    (switch Utilities|FlowControl|Switch|SwitchonExperimentType (Variables|Default|GetExperimentType)
      (:NewEnumerator0
        (bind _asbp_moon_experiemnt (Utilities|Casting|CastToBP_MoonExperiemnt _array_element))
        (Default|SetMoonphasesView _asbp_moon_experiemnt (Variables|Default|GetMoonphasesView)))
      (:NewEnumerator1
        (bind _asbp_binary_experiment (Utilities|Casting|CastToBP_BinaryExperiment _array_element))
        (Default|SetBinaryView _asbp_binary_experiment (Variables|Default|GetBinaryView)))
      (:NewEnumerator2
        (bind _asbp_frequency_experiment (Utilities|Casting|CastToBP_FrequencyExperiment _array_element))
        (Default|SetFrequencyView _asbp_frequency_experiment (Variables|Default|GetFrequencyView))))))

(fn SetMostDifficultExperimentFinished
  (switch Utilities|FlowControl|Switch|SwitchonExperimentDifficulty (Variables|Default|GetChosenDifficulty)
    (:NewEnumerator1
      (if (not (Utilities|Enum|Equal(Enum) (Variables|Default|GetMostDifficultExperimentThatsFinished) "NewEnumerator2"))
        (Variables|Default|SetMostDifficultExperimentThatsFinished "NewEnumerator1")))
    (:NewEnumerator2
      (Variables|Default|SetMostDifficultExperimentThatsFinished "NewEnumerator2"))))